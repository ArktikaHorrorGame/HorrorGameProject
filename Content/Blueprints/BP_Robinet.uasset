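; Faucet actor that, when activated, plays a metal sound and emits an AI-audible noise attributed to the player.
; ObjectActivate runs once through a DoOnce, calling the water spawn, sound, wide-range noise at AIPosition and a debug print.
; ObjectDesactivate calls the water despawn and re-arms the DoOnce.
; The water spawn and despawn events have empty bodies in this graph.
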(event Custom|Despawn_Water)

(event Custom|Spawn_Water)

(event EventBeginPlay)

(event Collision|EventActorBeginOverlap
  (params (OtherActor :type Actor%20Object%20Reference)))

(event EventTick
  (params (DeltaSeconds :type Float%20%28single-precision%29)))

(event EventObjectDesactivate
  (CallFunction|DespawnWater)
  (Utilities|FlowControl|DoOnce false) ; enters at Reset
)

(event EventObjectActivate
  (Utilities|FlowControl|DoOnce false
    (:Completed
      (CallFunction|SpawnWater)
      (Audio|PlaySoundatLocation "/Game/Blueprints/Audio/Footsteps/Metal_02.Metal_02" (Transformation|GetWorldLocation (Variables|Default|GetStaticMeshComponent1)) "0, 0, 0" 1.0 1.0 0.0 0 0 0 0)
      (Class|AISenseHearing|ReportNoiseEvent (Transformation|GetWorldLocation (Variables|Default|GetAI%20Position)) 1.0 (Game|GetPlayerCharacter 0) 1e+04 "None")
      (Development|PrintString "Robinet"))))

(fn ConstructionScript)