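; BP_Wheel_Key is a key pickup that unlocks a wheel attached to a door (Porte).
; On Interaction, it sets HasKey on the door, makes the BP_Wheel in the door's child actor component grabbable, then destroys itself.
; A sphere overlap drives the mesh's Highlight material parameter, turning the highlight on when overlap begins and off when it ends.
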(event OnComponentBeginOverlap(Sphere)
  (params (OverlappedComponent :type Primitive%20Component%20Object%20Reference) (OtherActor :type Actor%20Object%20Reference) (OtherComp :type Primitive%20Component%20Object%20Reference) (OtherBodyIndex :type Integer) (bFromSweep :type Boolean) (SweepResult :type Hit%20Result%20Structure%20%28by%20ref%29))
  (Rendering|Material|SetScalarParameterValueonMaterials (Variables|Default|GetStaticMesh) "Highlight" 3.0))

(event OnComponentEndOverlap(Sphere)
  (params (OverlappedComponent :type Primitive%20Component%20Object%20Reference) (OtherActor :type Actor%20Object%20Reference) (OtherComp :type Primitive%20Component%20Object%20Reference) (OtherBodyIndex :type Integer))
  (Rendering|Material|SetScalarParameterValueonMaterials (Variables|Default|GetStaticMesh) "Highlight" 0.0))

(event EventInteraction
  (bind _porte (Variables|Default|GetPorte))
  (Variables|/Game/Blueprints/BP_Object/BP_BaseObject.BP_BaseObject_C|SetHas%20Key%20? _porte true)
  (Variables|/Game/Blueprints/BP_Object/BP_Wheel.BP_Wheel_C|SetCan_Be_Grab? (.AsBP%20Wheel (Utilities|Casting|CastToBP_Wheel (Variables|/Script/Engine.ChildActorComponent|GetChildActor (Variables|/Game/Blueprints/BP_Porte.BP_Porte_C|GetBP_Wheel _porte)))) true)
  (Actor|DestroyActor))

(fn ConstructionScript)