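; Audio trigger actor that fades conduit monster music in and out as the player moves through the level.
; When BP_Player first enters the start box, the cue plays and the FonduMusique timeline drives its volume multiplier from silent to full.
; When the player first enters the end box, the same timeline reverses from its end at a faster rate to fade the volume back down.
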(event OnComponentBeginOverlap(BoxDebutMusique)
  (params (OverlappedComponent :type Primitive%20Component%20Object%20Reference) (OtherActor :type Actor%20Object%20Reference) (OtherComp :type Primitive%20Component%20Object%20Reference) (OtherBodyIndex :type Integer) (bFromSweep :type Boolean) (SweepResult :type Hit%20Result%20Structure%20%28by%20ref%29))
  (bind _bruit_de_monstre_conduit_musique__1__cue (Variables|Default|Getbruit-de-monstre-conduit-musique-_1__Cue))
  (Utilities|Casting|CastToBP_Player OtherActor)
  (Utilities|FlowControl|DoOnce false
    (:Completed
      (Audio|Components|Audio|Play _bruit_de_monstre_conduit_musique__1__cue 0.0)
      (bind _lerp (Timeline|FonduMusique PlayFromStart)
        (:Update
          (Audio|Components|Audio|SetVolumeMultiplier _bruit_de_monstre_conduit_musique__1__cue (Math|Float|Lerp 0.0 1.0 _lerp) :!class /Script/Engine.AudioComponent))))))

(event OnComponentBeginOverlap(BoxFinMusique)
  (params (OverlappedComponent :type Primitive%20Component%20Object%20Reference) (OtherActor :type Actor%20Object%20Reference) (OtherComp :type Primitive%20Component%20Object%20Reference) (OtherBodyIndex :type Integer) (bFromSweep :type Boolean) (SweepResult :type Hit%20Result%20Structure%20%28by%20ref%29))
  (Utilities|Casting|CastToBP_Player OtherActor)
  (Utilities|FlowControl|DoOnce false
    (:Completed
      (Components|Timeline|SetPlayRate (Variables|Default|GetFonduMusique) 1.5)
      (bind _lerp (Timeline|FonduMusique ReverseFromEnd)
        (:Update
          (Audio|Components|Audio|SetVolumeMultiplier (Variables|Default|Getbruit-de-monstre-conduit-musique-_1__Cue) (Math|Float|Lerp 0.0 1.0 _lerp) :!class /Script/Engine.AudioComponent))))))

(fn ConstructionScript)