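; Cinematic pipe actor that stages a steam jet knocking the player back and destroying a wall; despite its name, it plays no audio.
; Events toggle the steam Niagara lifetime and switch the wall to overlap.
; Knockback runs a timeline scaled by KnockBackTime, moving the player to an actor-relative reference point and triggering wall destruction once.
; Push_Player is an empty stub, and its launch logic is disconnected.
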(event Custom|Spawn%20Steam%20Jet
  (bind _steamjetref (Variables|Default|GetSteamjetRef))
  (Effects|Components|ParticleSystem|SetFloatParameter (Variables|/Game/Jules/BluePrint/Toxic_Gaz.Toxic_Gaz_C|GetNiagara _steamjetref) "LifeTime" 4.0)
  (Variables|/Game/Jules/BluePrint/Toxic_Gaz.Toxic_Gaz_C|SetLT_Distance _steamjetref 0.0))

(event Custom|Knockback
  (bind _knockback_firstref (Variables|Default|GetKnockback_FirstRef))
  (Components|Timeline|SetPlayRate (Variables|Default|GetKnockback%20Player) (/ 1.0 (Variables|Default|GetKnockBack_Time)))
  (Timeline|Knockback%20Player Play
    (:Update
      (Utilities|FlowControl|Sequence
        (:then_0
          (Transformation|SetWorldLocationAndRotation (Variables|/Script/Engine.Actor|GetRootComponent (Game|GetPlayerCharacter 0)) (Math|Transform|TransformLocation (Transformation|GetActorTransform) (.location _knockback_firstref)) (.rotation _knockback_firstref) false false))
        (:then_1
          (Utilities|FlowControl|DoOnce false
            (:Completed
              (Default|DestroyWall (Variables|Default|GetWall_Ref)))))))))

(event Custom|NoCollision%20Wall
  (bind _wall_ref (Variables|Default|GetWall_Ref))
  (Collision|SetCollisionEnabled (Variables|/Game/Blueprints/Cinematics/Grid_Explosion.Grid_Explosion_C|GetBox _wall_ref) "QueryOnly")
  (Collision|SetCollisionResponsetoChannel (Variables|/Game/Blueprints/Cinematics/Grid_Explosion.Grid_Explosion_C|GetStaticMeshComponent0 _wall_ref) "ECC_Pawn" "ECR_Overlap"))

(event Custom|Push_Player
  ;[1 0.5198 0.1382] Probably replace that by a Timeline or make it great depending on the direction between the player and the PushPoint ref
)

(event EventBeginPlay
  (bind _steamjetref (Variables|Default|GetSteamjetRef))
  (Variables|Default|SetPushPoint_Ref (Math|Transform|MakeTransform "0.000000,1800.000000,0.000000" "0, 0, 0" "1.000000,1.000000,1.000000"))
  (Variables|Default|SetSteamJet_Ref (Math|Transform|MakeTransform "0.000000,142.000000,0.000000" "0, 0, 0" "1.000000,1.000000,1.000000"))
  (Variables|Default|SetKnockback_FirstRef (Math|Transform|MakeTransform "0.000000,2650.000000,0.000000" "0, 0, 0" "1.000000,1.000000,1.000000"))
  (Variables|Default|SetHeadRotation_Ref (Math|Transform|MakeTransform "0.000000,2650.000000,900.000000" "0, 0, 0" "1.000000,1.000000,1.000000"))
  (Effects|Components|ParticleSystem|SetFloatParameter (Variables|/Game/Jules/BluePrint/Toxic_Gaz.Toxic_Gaz_C|GetNiagara _steamjetref) "LifeTime" 0.0)
  (Variables|/Game/Jules/BluePrint/Toxic_Gaz.Toxic_Gaz_C|SetLT_Distance _steamjetref 0.0))

(event Collision|EventActorBeginOverlap
  (params (OtherActor :type Actor%20Object%20Reference)))

(event EventTick
  (params (DeltaSeconds :type Float%20%28single-precision%29)))

(fn ConstructionScript)