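; Cinematic manager Blueprint for a push-the-box sequence, apparently unfinished.
; Walk and EndCinematic events drive the wooden crate reference, with the latter restoring player input and teleporting the player.
; The trigger logic that disables input and schedules these events on timers is disconnected, and StartCinematic only looks up a LevelInstance actor.
; The construction script prints a debug string and calls the empty CinematicPushtheBox event.
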(event Custom|StartCinematic
  (Actor|GetActorOfClass "/Script/Engine.LevelInstance"))

(event Custom|End%20Cinematic
  (Input|EnableInput (.AsBP%20Player (Utilities|Casting|CastToBP_Player (Game|GetPlayerCharacter 0))) 0)
  (Default|TpPlayerEndCinematic (Variables|Default|GetWoodenCrate_Ref)))

(event Custom|Walk
  (bind _woodencrate_ref (Variables|Default|GetWoodenCrate_Ref))
  (Default|Walk _woodencrate_ref)
  (Default|HeadDown _woodencrate_ref))

(event Custom|Cinematic%20Push%20the%20Box)

(event EventBeginPlay)

(event Collision|EventActorBeginOverlap
  (params (OtherActor :type Actor%20Object%20Reference)))

(event EventTick
  (params (DeltaSeconds :type Float%20%28single-precision%29)))

(fn ConstructionScript
  (Development|PrintString "Hello" false)
  (CallFunction|CinematicPushtheBox))