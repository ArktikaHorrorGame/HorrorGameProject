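; Trigger actor for the pipe trap cinematic, in which a pipe explosion knocks the player down and they slowly get back up.
; On overlap, input is disabled while the player walks and looks at the pipe, then a timer chain of nine parts runs the sequence.
; Timelines drive control rotation and spring arm offset for the fall and recovery, layered with camera shakes, fades, white flash and post-process double vision.
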(event OnComponentBeginOverlap(Box)
  (params (OverlappedComponent :type Primitive%20Component%20Object%20Reference) (OtherActor :type Actor%20Object%20Reference) (OtherComp :type Primitive%20Component%20Object%20Reference) (OtherBodyIndex :type Integer) (bFromSweep :type Boolean) (SweepResult :type Hit%20Result%20Structure%20%28by%20ref%29))
  ;[1 1 1] Pipe trap cinematic
  (Utilities|Casting|CastToBP_Player OtherActor)
  (if (Variables|/Game/Blueprints/Cinematics/PipeTrap/BP_Activate_PlayerFall.BP_Activate_PlayerFall_C|GetEnableCinematic? (Variables|Default|GetActivate_Player_Ref))
    (Utilities|FlowControl|DoOnce false
      (:Completed
        (Utilities|FlowControl|Sequence
          (:then_0
            (Default|Footstep-Headshake (.AsBP%20Player (Utilities|Casting|CastToBP_Player (Game|GetPlayerCharacter 0))) "NewEnumerator0"))
          (:then_1
            (CallFunction|WalkWhileWatchingPipe)
            (CallFunction|CameraShakes)
            (CallFunction|WatchthePipe)
            (Default|NoCollisionWall (Variables|Default|GetPipes%20Sound%20Ref))
            (Utilities|Time|SetTimerbyEvent (delegate Custom|Part%201) 0.85)))))))

(event Custom|Reset_WhiteFlash
  (bind _returnvalue (Game|GetPlayerCharacter 0))
  (bind _asbp_player (Utilities|Casting|CastToBP_Player _returnvalue))
  (bind _camera (Variables|/Game/Blueprints/BP_Player.BP_Player_C|GetCamera _asbp_player))
  ;[1 1 1] Pipe trap cinematic
  ;;[0 0 0] Stop White Flash
  (bind _structout (Utilities|Struct|SetmembersinPostProcessSettings (Variables|/Script/Engine.CameraComponent|GetPostProcessSettings _camera) 0.675))
  (Variables|/Script/Engine.CameraComponent|SetPostProcessSettings _camera _structout))

(event Custom|Camera%20Shakes
  ;[1 1 1] Pipe trap cinematic
  ;;[0.4844 0.4266 0.08959] Camera Shakes
  (Camera|PlayWorldCameraShake "/Game/Blueprints/Widget/Camera_Shake.Camera_Shake_C" (Transformation|GetActorLocation) 0.0 5e+02)
  (Development|PrintString "Hello"))

(event Custom|Mid%20Stand%20Up
  ;[1 1 1] Pipe trap cinematic
  ;;[0.9686 0.1529 1] Mid Stand Up
  (Components|Timeline|SetPlayRate (Variables|Default|GetMid%20Standing%20Up) (/ 1.0 (Variables|Default|GetLooking%20Up)))
  (bind _newtrack_0 (Timeline|Mid%20Standing%20Up Play)
    (:Update
      (Pawn|SetControlRotation (Game|GetPlayerController 0) (Math|Rotator|Lerp(Rotator) (Variables|Default|GetLook%20Forward) "-45.000000,90.000000,0.000000" _newtrack_0)))))

(event Custom|Camera%20Shakes%20Fall
  ;[1 1 1] Pipe trap cinematic
  ;;[0.4844 0.4266 0.08959] Camera Shakes
  (Camera|PlayWorldCameraShake "/Game/Blueprints/Widget/Camera_Shake_Fall.Camera_Shake_Fall_C" (Transformation|GetActorLocation) 0.0 5e+02)
  (Development|PrintString "Hello"))

(event Custom|Start%20Stand%20Up
  (bind _returnvalue (Transformation|GetActorRotation))
  (bind (_roll _pitch _yaw) (Math|Rotator|BreakRotator _returnvalue))
  ;[1 1 1] Pipe trap cinematic
  ;;[0.9686 0.1529 1] Start Stand Up
  (Components|Timeline|SetPlayRate (Variables|Default|GetStart%20Standing%20Up) (/ 1.0 (Variables|Default|GetStand%20Up)))
  (bind _newtrack_0 (Timeline|Start%20Standing%20Up Play)
    (:Update
      (Pawn|SetControlRotation (Game|GetPlayerController 0) (Math|Rotator|Lerp(Rotator) (Variables|Default|GetHead's%20on%20Ground) (Math|Rotator|MakeRotator (- _roll 89.0) (- _pitch 9e+01) (+ _yaw 1.8e+02)) _newtrack_0 true))
      (Variables|Default|SetLook%20Forward (Math|Rotator|Lerp(Rotator) (Variables|Default|GetHead's%20on%20Ground) (Math|Rotator|MakeRotator (- _roll 89.0) (- _pitch 9e+01) (+ _yaw 1.8e+02)) _newtrack_0 true)))))

(event Custom|End%20Stand%20Up
  ;[1 1 1] Pipe trap cinematic
  ;;[0.9686 0.1529 1] End Stand Up
  (Components|Timeline|SetPlayRate (Variables|Default|GetEnd%20Standing%20Up) (/ 1.0 (Variables|Default|GetStand%20Up)))
  (bind _newtrack_0 (Timeline|End%20Standing%20Up Play)
    (:Update
      (Variables|/Script/Engine.SpringArmComponent|SetTargetOffset (Variables|/Game/Blueprints/BP_Player.BP_Player_C|GetSpringArm (.AsBP%20Player (Utilities|Casting|CastToBP_Player (Game|GetPlayerCharacter 0)))) (Math|Vector|Lerp(Vector) (Variables|Default|GetCameraOnGround) (Variables|Default|GetOriginal%20Target%20Offset) _newtrack_0))
      (Components|Timeline|SetPlayRate (Variables|Default|GetNodding) (/ 1.0 (Variables|Default|GetNodding%20Head)))
      (bind _newtrack_0_2 (Timeline|Nodding Play)
        (:Update
          (Pawn|SetControlRotation (Game|GetPlayerController 0) (Math|Rotator|Lerp(Rotator) "0.000000,90.000000,0.000000" "-30.000000,90.000000,0.000000" _newtrack_0_2)))))))

(event Custom|FlashBang%20Effect
  (bind _returnvalue (Game|GetPlayerCharacter 0))
  (bind _asbp_player (Utilities|Casting|CastToBP_Player _returnvalue))
  (bind _camera (Variables|/Game/Blueprints/BP_Player.BP_Player_C|GetCamera _asbp_player))
  (bind _postprocesssettings (Variables|/Script/Engine.CameraComponent|GetPostProcessSettings _camera))
  (bind _weightedblendables (Utilities|Struct|BreakPostProcessSettings _postprocesssettings))
  (bind _array (Utilities|Struct|BreakWeightedBlendables _weightedblendables))
  ;[1 1 1] Pipe trap cinematic
  ;;[1 0.8659 0.3512] Flashbang Effect
  (Components|Timeline|SetPlayRate (Variables|Default|GetDouble%20Image%20Effect) (/ 1.0 (Variables|Default|GetDouble%20Image%20Time)))
  (bind _newtrack_0 (Timeline|Double%20Image%20Effect Play)
    (:Update
      (Utilities|Array|SetArrayElem _array 0 (Utilities|Array|Get(acopy) (Utilities|Array|MakeArray (Utilities|Struct|MakeWeightedBlendable _newtrack_0 "/Game/Jules/PostProcessMAterial/M_PostProcess_FlashBang_Inst.M_PostProcess_FlashBang_Inst"))))
      (Utilities|FlowControl|Delay 1e+01)
      (Utilities|Array|SetArrayElem _array 0 (Utilities|Array|Get(acopy) (Utilities|Array|MakeArray (Utilities|Struct|MakeWeightedBlendable 0.0 "/Game/Jules/PostProcessMAterial/M_PostProcess_FlashBang_Inst.M_PostProcess_FlashBang_Inst")))))))

(event Custom|Destroy%20Timeline
  (bind _returnvalue (Game|GetPlayerCharacter 0))
  (bind _returnvalue_2 (Game|GetPlayerController 0))
  (bind _asbp_player (Utilities|Casting|CastToBP_Player _returnvalue))
  (bind _springarm (Variables|/Game/Blueprints/BP_Player.BP_Player_C|GetSpringArm _asbp_player))
  ;[1 1 1] Pipe trap cinematic
  ;;[0.2018 0.365 0.625] Watch Pipe
  (bind _rotation (Timeline|Watch%20Pipe Stop)
    (:Update
      (Pawn|SetControlRotation _returnvalue_2 (Math|Rotator|Lerp(Rotator) (Pawn|GetControlRotation _returnvalue_2 :!class /Script/Engine.Controller) (Math|Rotator|Lerp(Rotator) (Transformation|GetWorldRotation _springarm) (Math|Rotator|FindLookatRotation (Transformation|GetWorldLocation _springarm) (Transformation|GetWorldLocation (Variables|/Game/Blueprints/Cinematics/PipeTrap/BP_Pipes_Sound.BP_Pipes_Sound_C|GetCube (Variables|Default|GetPipes%20Sound%20Ref)))) _rotation true) _rotation true))
      (Input|DisableInput (.AsBP%20Player (Utilities|Casting|CastToBP_Player (Game|GetPlayerCharacter 0))) 0))
    (:Finished
      (Development|PrintString "DONEEEE"))))

(event Custom|Walk%20while%20Watching%20Pipe
  (bind _returnvalue (Game|GetPlayerCharacter 0))
  (bind _rootcomponent (Variables|/Script/Engine.Actor|GetRootComponent _returnvalue))
  (bind _returnvalue_2 (Transformation|GetWorldLocation _rootcomponent))
  (bind _returnvalue_3 (Transformation|GetWorldLocation _rootcomponent))
  ;[1 1 1] Pipe trap cinematic
  ;;[0.6131 0.3106 0.6198] Walking
  (Components|Timeline|SetPlayRate (Variables|Default|GetWalking) (/ 1.0 (Variables|Default|GetWalking%20Speed)))
  (Input|DisableInput (.AsBP%20Player (Utilities|Casting|CastToBP_Player (Game|GetPlayerCharacter 0))) 0)
  (bind _speed (Timeline|Walking Play)
    (:Update
      (Transformation|SetActorLocation (Game|GetPlayerCharacter 0) (Math|Vector|Lerp(Vector) (Math|Vector|MakeVector (.x _returnvalue_2) (.y _returnvalue_2) (.z _returnvalue_2)) (Math|Vector|MakeVector (.x _returnvalue_3) (- (.y _returnvalue_3) 1.0) (.z _returnvalue_3)) _speed) false false))))

(event Custom|FadeOut
  ;[1 1 1] Pipe trap cinematic
  ;;[0 0 0] Fade In / Fade Out
  (CameraFades|StartCameraFade :self (Game|GetPlayerCameraManager 0) :FromAlpha 1.0 :Duration 4.3))

(event Custom|WhiteFlash
  (bind _returnvalue (Game|GetPlayerCharacter 0))
  (bind _asbp_player (Utilities|Casting|CastToBP_Player _returnvalue))
  (bind _camera (Variables|/Game/Blueprints/BP_Player.BP_Player_C|GetCamera _asbp_player))
  ;[1 1 1] Pipe trap cinematic
  ;;[1 1 1] White Flash
  (Components|Timeline|SetPlayRate (Variables|Default|GetWhiteScreen) (/ 1.0 (Variables|Default|GetWhiteScreen%20Time)))
  (bind _newtrack_0 (Timeline|WhiteScreen Play)
    (:Update
      (bind _structout (Utilities|Struct|SetmembersinPostProcessSettings (Variables|/Script/Engine.CameraComponent|GetPostProcessSettings _camera) (* _newtrack_0 5e+02)))
      (Variables|/Script/Engine.CameraComponent|SetPostProcessSettings _camera _structout))))

(event Custom|Trying%20to%20Stand%20Up
  (bind _head_s_on_ground (Variables|Default|GetHead's%20on%20Ground))
  ;[1 1 1] Pipe trap cinematic
  ;;[0.108 0.3385 0.2259] Trying To Stand Up
  (Components|Timeline|SetPlayRate (Variables|Default|GetTrying%20to%20Wake%20Up) (/ 1.0 (Variables|Default|GetTrying%20Time)))
  (bind _newtrack_0 (Timeline|Trying%20to%20Wake%20Up Play)
    (:Update
      (Pawn|SetControlRotation (Game|GetPlayerController 0) (Math|Rotator|Lerp(Rotator) (Variables|Default|GetHead's%20on%20Ground) (Math|Rotator|MakeRotator (- (.roll _head_s_on_ground) 5.0) (- (.pitch _head_s_on_ground) 5.0) (.yaw _head_s_on_ground)) _newtrack_0 true)))))

(event Custom|Stop%20Lock%20Look
  ;[1 1 1] Pipe trap cinematic
  ;;[0.03913 0.25 0.02986] Stop Lock Look
  (Utilities|FlowControl|RetriggerableDelay 0.2)
  (Variables|Default|SetGrippedd false)
  (bind _asbp_player (Utilities|Casting|CastToBP_Player (Game|GetPlayerCharacter 0)))
  (Pawn|SetControlRotation (Game|GetPlayerController 0) (Class|SpringArmComponent|GetTargetRotation (Variables|/Game/Blueprints/BP_Player.BP_Player_C|GetSpringArm _asbp_player)))
  (Input|EnableInput (.AsBP%20Player (Utilities|Casting|CastToBP_Player (Game|GetPlayerCharacter 0))) 0))

(event Custom|Part%201
  ;[1 1 1] Pipe trap cinematic
  (Default|SpawnSteamJet (Variables|Default|GetPipes%20Sound%20Ref))
  (Default|Explosion (Variables|Default|GetPipes%20Sound%20Ref))
  (Utilities|FlowControl|Sequence
    (:then_0
      (Utilities|Time|SetTimerbyFunctionName 0 "Flash Bang Effect" 0.4))
    (:then_1
      (Utilities|Time|SetTimerbyEvent (delegate Custom|Part%202) 0.5))))

(event Custom|Part%202
  ;[1 1 1] Pipe trap cinematic
  (CallFunction|WhiteFlash)
  (Default|Knockback (Variables|Default|GetPipes%20Sound%20Ref))
  (CallFunction|LoseIteminHand)
  (CallFunction|FallingRotation)
  (CallFunction|CameraShakesFall)
  (Utilities|FlowControl|Sequence
    (:then_0
      (CallFunction|CameraonGround))
    (:then_1
      (Utilities|Time|SetTimerbyEvent (delegate Custom|Part%203) 0.15))))

(event Custom|Part%203
  ;[1 1 1] Pipe trap cinematic
  (CallFunction|TiltedCameraGround)
  (Utilities|Time|SetTimerbyEvent (delegate Custom|Part%204) 1.3))

(event Custom|Part%204
  ;[1 1 1] Pipe trap cinematic
  (CallFunction|TryingtoStandUp)
  (Utilities|Time|SetTimerbyEvent (delegate Custom|Part%205) 1.3))

(event Custom|Part%205
  ;[1 1 1] Pipe trap cinematic
  (CallFunction|Fadein/FadeOut)
  (Utilities|FlowControl|Sequence
    (:then_0
      (Utilities|Time|SetTimerbyFunctionName 0 "Reset White Flash" 3.5))
    (:then_1
      (Utilities|Time|SetTimerbyEvent (delegate Custom|Part%206) 5.5))))

(event Custom|Part%206
  ;[1 1 1] Pipe trap cinematic
  (CallFunction|StartStandUp)
  (Utilities|Time|SetTimerbyEvent (delegate Custom|Part%207) 1.8))

(event Custom|Part%207
  ;[1 1 1] Pipe trap cinematic
  (CallFunction|MidStandUp)
  (Utilities|Time|SetTimerbyEvent (delegate Custom|Part%208) 1.5))

(event Custom|Part%208
  ;[1 1 1] Pipe trap cinematic
  (CallFunction|EndStandUp)
  (Utilities|Time|SetTimerbyEvent (delegate Custom|Part%209) 2.2))

(event Custom|Part%209
  ;[1 1 1] Pipe trap cinematic
  (Input|EnableInput (.AsBP%20Player (Utilities|Casting|CastToBP_Player (Game|GetPlayerCharacter 0))) 0)
  (CallFunction|StopLockLook))

(event Custom|Camera%20On%20Ground
  (bind _returnvalue (Game|GetPlayerCharacter 0))
  (bind _asbp_player (Utilities|Casting|CastToBP_Player _returnvalue))
  (bind _springarm (Variables|/Game/Blueprints/BP_Player.BP_Player_C|GetSpringArm _asbp_player))
  ;[1 1 1] Pipe trap cinematic
  ;;[0.03635 0.02151 0.125] Camera On Ground
  (bind _output_get (Variables|/Script/Engine.SpringArmComponent|SetTargetOffset _springarm (Math|Vector|MakeVector (.x (Variables|/Script/Engine.SpringArmComponent|GetTargetOffset _springarm)) (.y (Variables|/Script/Engine.SpringArmComponent|GetTargetOffset _springarm)) -95.0)))
  (Variables|Default|SetCameraOnGround _output_get))

(event Custom|Watch_the_Pipe
  (bind _returnvalue (Game|GetPlayerCharacter 0))
  (bind _returnvalue_2 (Game|GetPlayerController 0))
  (bind _asbp_player (Utilities|Casting|CastToBP_Player _returnvalue))
  (bind _springarm (Variables|/Game/Blueprints/BP_Player.BP_Player_C|GetSpringArm _asbp_player))
  ;[1 1 1] Pipe trap cinematic
  ;;[0.2018 0.365 0.625] Watch Pipe
  (Components|Timeline|SetPlayRate (Variables|Default|GetWatch%20Pipe) (/ 1.0 (Variables|Default|GetTime_watch_Pipe)))
  (Utilities|Time|SetTimerbyEvent (delegate Custom|Destroy%20Timeline) 2.0)
  (bind _rotation (Timeline|Watch%20Pipe Play)
    (:Update
      (Pawn|SetControlRotation _returnvalue_2 (Math|Rotator|Lerp(Rotator) (Pawn|GetControlRotation _returnvalue_2 :!class /Script/Engine.Controller) (Math|Rotator|Lerp(Rotator) (Transformation|GetWorldRotation _springarm) (Math|Rotator|FindLookatRotation (Transformation|GetWorldLocation _springarm) (Transformation|GetWorldLocation (Variables|/Game/Blueprints/Cinematics/PipeTrap/BP_Pipes_Sound.BP_Pipes_Sound_C|GetCube (Variables|Default|GetPipes%20Sound%20Ref)))) _rotation true) _rotation true))
      (Input|DisableInput (.AsBP%20Player (Utilities|Casting|CastToBP_Player (Game|GetPlayerCharacter 0))) 0))
    (:Finished
      (Development|PrintString "DONEEEE"))))

(event Custom|Tilted%20Camera%20Ground
  (bind _returnvalue (Transformation|GetActorRotation))
  (bind (_roll _pitch _yaw) (Math|Rotator|BreakRotator _returnvalue))
  ;[1 1 1] Pipe trap cinematic
  ;;[0.2812 0.1504 0.08476] Tilted Camera Ground
  (Components|Timeline|SetPlayRate (Variables|Default|Gettilted%20camera) (/ 1.0 (Variables|Default|GetTilted%20Camera%20Rotation)))
  (bind _newtrack_0 (Timeline|Tilted%20Camera Play)
    (:Update
      (Pawn|SetControlRotation (Game|GetPlayerController 0) (Math|Rotator|Lerp(Rotator) (Variables|Default|GetHead's%20Up) (Math|Rotator|MakeRotator (- _roll 315.0) _pitch (- _yaw 3.6e+02)) _newtrack_0 true))
      (Variables|Default|SetHead's%20on%20Ground (Math|Rotator|Lerp(Rotator) (Variables|Default|GetHead's%20Up) (Math|Rotator|MakeRotator (- _roll 315.0) _pitch (- _yaw 3.6e+02)) _newtrack_0 true)))))

(event Custom|Lock%20look
  ;[1 1 1] Pipe trap cinematic
  ;;[0.2708 0.007835 0] Lock Look
  (bind _asbp_player (Utilities|Casting|CastToBP_Player (Game|GetPlayerCharacter 0)))
  (Variables|Default|GetPipes%20Sound%20Ref
    (:then
      (Pawn|SetControlRotation (Game|GetPlayerController 0) (Math|Rotator|FindLookatRotation (Transformation|GetWorldLocation (Variables|/Game/Blueprints/BP_Player.BP_Player_C|GetSpringArm _asbp_player)) (Transformation|GetWorldLocation (Variables|/Game/Blueprints/Cinematics/PipeTrap/BP_Pipes_Sound.BP_Pipes_Sound_C|GetCube (Variables|Default|GetPipes%20Sound%20Ref))))))
    (:else)))

(event Custom|Lose%20Item%20In%20Hand
  ;[1 1 1] Pipe trap cinematic
  ;;[0.401 0.1284 0] Lose item In Hand
  (Default|Release (.AsBP%20Player (Utilities|Casting|CastToBP_Player (Game|GetPlayerCharacter 0)))))

(event Custom|Fade%20In%20/%20Fade%20Out
  ;[1 1 1] Pipe trap cinematic
  ;;[0 0 0] Fade In / Fade Out
  (CameraFades|StartCameraFade :self (Game|GetPlayerCameraManager 0) :ToAlpha 1.0 :Duration 1.75 :bShouldFadeAudio true :bHoldWhenFinished true)
  (Utilities|Time|SetTimerbyEvent (delegate Custom|FadeOut) 3.5))

(event Custom|Falling_Rotation
  (bind _returnvalue (Game|GetPlayerCharacter 0))
  (bind _pipes_sound_ref (Variables|Default|GetPipes%20Sound%20Ref))
  (bind _asbp_player (Utilities|Casting|CastToBP_Player _returnvalue))
  (bind _cube (Variables|/Game/Blueprints/Cinematics/PipeTrap/BP_Pipes_Sound.BP_Pipes_Sound_C|GetCube _pipes_sound_ref))
  (bind _returnvalue_2 (Transformation|GetWorldLocation _cube))
  (bind _springarm (Variables|/Game/Blueprints/BP_Player.BP_Player_C|GetSpringArm _asbp_player))
  (bind _returnvalue_3 (Transformation|GetWorldLocation _springarm))
  (bind _returnvalue_4 (Math|Rotator|FindLookatRotation _returnvalue_3 _returnvalue_2))
  ;[1 1 1] Pipe trap cinematic
  ;;[0.2964 1 0.7018] Falling Rotation
  (Components|Timeline|SetPlayRate (Variables|Default|GetHead_Rotation) (/ 1.0 (Variables|Default|GetTime_Head_Rotation)))
  (bind _rotation (Timeline|Head_Rotation Play)
    (:Update
      (Pawn|SetControlRotation (Game|GetPlayerController 0) (Math|Rotator|Lerp(Rotator) (Math|Rotator|FindLookatRotation _returnvalue_3 _returnvalue_2) (Math|Rotator|MakeRotator (.roll _returnvalue_4) 9e+01 (.yaw _returnvalue_4)) _rotation true))
      (Variables|Default|SetHead's%20Up (Math|Rotator|Lerp(Rotator) (Math|Rotator|FindLookatRotation _returnvalue_3 _returnvalue_2) (Math|Rotator|MakeRotator (.roll _returnvalue_4) 9e+01 (.yaw _returnvalue_4)) _rotation true)))))

(event EventBeginPlay
  ;[1 1 1] Pipe trap cinematic
  (Actor|Tick|SetActorTickEnabled false)
  (Variables|Default|SetCurrent%20Rotation (Transformation|GetActorRotation))
  (Variables|Default|SetOriginal%20Target%20Offset (Variables|/Script/Engine.SpringArmComponent|GetTargetOffset (Variables|/Game/Blueprints/BP_Player.BP_Player_C|GetSpringArm (.AsBP%20Player (Utilities|Casting|CastToBP_Player (Game|GetPlayerCharacter 0))))))
  (Variables|Default|SetPlayerSpeed (Transformation|GetWorldLocation (Variables|/Script/Engine.Actor|GetRootComponent (Game|GetPlayerCharacter 0)))))

(event EventTick
  (params (DeltaSeconds :type Float%20%28single-precision%29))
  ;[1 1 1] Pipe trap cinematic
  (if (Variables|Default|GetGrippedd)
    (CallFunction|LockLook)))

(fn ConstructionScript)