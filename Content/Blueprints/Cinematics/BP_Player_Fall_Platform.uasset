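; Trigger-box actor for a one-shot cinematic in which a steam pipe knocks the player down, gated by ActivatePlayerRef's EnableCinematic flag.
; On overlap it disables input and turns the view to the pipe, then fires steam and knockback and releases the held item.
; Timelines lerp control rotation upward and into a tilt while the spring arm offset drops to ground level.
; Camera and input restore logic exists but is unwired.
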(event OnComponentBeginOverlap(Box)
  (params (OverlappedComponent :type Primitive%20Component%20Object%20Reference) (OtherActor :type Actor%20Object%20Reference) (OtherComp :type Primitive%20Component%20Object%20Reference) (OtherBodyIndex :type Integer) (bFromSweep :type Boolean) (SweepResult :type Hit%20Result%20Structure%20%28by%20ref%29))
  (bind _pipes_sound_ref (Variables|Default|GetPipes%20Sound%20Ref))
  ;[1 1 1] Comment
  (if (Variables|/Game/Blueprints/Cinematics/BP_Activate_PlayerFall.BP_Activate_PlayerFall_C|GetEnableCinematic? (Variables|Default|GetActivate_Player_Ref))
    (Utilities|FlowControl|DoOnce false
      (:Completed
        (CallFunction|WatchthePipe)
        (Default|NoCollisionWall (Variables|Default|GetPipes%20Sound%20Ref))
        (Utilities|FlowControl|Delay 1.0)
        (Default|SpawnSteamJet _pipes_sound_ref)
        (Utilities|FlowControl|Delay 0.5)
        (Default|Knockback _pipes_sound_ref)
        (CallFunction|LoseIteminHand)
        (CallFunction|FallingRotation)
        (Utilities|FlowControl|Sequence
          (:then_0
            (CallFunction|CameraonGround))
          (:then_1
            (Utilities|FlowControl|Delay 0.15)
            (CallFunction|TiltedCameraGround)))))))

(event Custom|Falling_Rotation
  (bind _returnvalue (Game|GetPlayerCharacter 0))
  (bind _pipes_sound_ref (Variables|Default|GetPipes%20Sound%20Ref))
  (bind _asbp_player (Utilities|Casting|CastToBP_Player _returnvalue))
  (bind _cube (Variables|/Game/Blueprints/Cinematics/BP_Pipes_Sound.BP_Pipes_Sound_C|GetCube _pipes_sound_ref))
  (bind _returnvalue_2 (Transformation|GetWorldLocation _cube))
  (bind _springarm (Variables|/Game/Blueprints/BP_Player.BP_Player_C|GetSpringArm _asbp_player))
  (bind _returnvalue_3 (Transformation|GetWorldLocation _springarm))
  (bind _returnvalue_4 (Math|Rotator|FindLookatRotation _returnvalue_3 _returnvalue_2))
  ;[1 1 1] Comment
  (Components|Timeline|SetPlayRate (Variables|Default|GetHead_Rotation) (/ 1.0 (Variables|Default|GetTime_Head_Rotation)))
  (bind _rotation (Timeline|Head_Rotation Play)
    (:Update
      (Pawn|SetControlRotation (Game|GetPlayerController 0) (Math|Rotator|Lerp(Rotator) (Math|Rotator|FindLookatRotation _returnvalue_3 _returnvalue_2) (Math|Rotator|MakeRotator (.roll _returnvalue_4) 9e+01 (.yaw _returnvalue_4)) _rotation true))
      (Variables|Default|SetHead's%20Up (Math|Rotator|Lerp(Rotator) (Math|Rotator|FindLookatRotation _returnvalue_3 _returnvalue_2) (Math|Rotator|MakeRotator (.roll _returnvalue_4) 9e+01 (.yaw _returnvalue_4)) _rotation true)))))

(event Custom|Normal%20Camera
  ;[1 1 1] Comment
  (Pawn|SetControlRotation (Game|GetPlayerController 0) (Variables|Default|GetCurrent%20Rotation))
  (Variables|/Script/Engine.SpringArmComponent|SetTargetOffset (Variables|/Game/Blueprints/BP_Player.BP_Player_C|GetSpringArm (.AsBP%20Player (Utilities|Casting|CastToBP_Player (Game|GetPlayerCharacter 0)))) (Variables|Default|GetOriginal%20Target%20Offset)))

(event Custom|Stop%20Lock%20Look
  ;[1 1 1] Comment
  (Utilities|FlowControl|RetriggerableDelay 0.2)
  (Variables|Default|SetGrippedd false)
  (bind _asbp_player (Utilities|Casting|CastToBP_Player (Game|GetPlayerCharacter 0)))
  (Pawn|SetControlRotation (Game|GetPlayerController 0) (Class|SpringArmComponent|GetTargetRotation (Variables|/Game/Blueprints/BP_Player.BP_Player_C|GetSpringArm _asbp_player)))
  (Input|EnableInput (.AsBP%20Player (Utilities|Casting|CastToBP_Player (Game|GetPlayerCharacter 0))) 0))

(event Custom|Camera%20On%20Ground
  (bind _returnvalue (Game|GetPlayerCharacter 0))
  (bind _asbp_player (Utilities|Casting|CastToBP_Player _returnvalue))
  (bind _springarm (Variables|/Game/Blueprints/BP_Player.BP_Player_C|GetSpringArm _asbp_player))
  ;[1 1 1] Comment
  (Variables|/Script/Engine.SpringArmComponent|SetTargetOffset _springarm (Math|Vector|MakeVector (.x (Variables|/Script/Engine.SpringArmComponent|GetTargetOffset _springarm)) (.y (Variables|/Script/Engine.SpringArmComponent|GetTargetOffset _springarm)) -95.0)))

(event Custom|Watch_the_Pipe
  (bind _returnvalue (Game|GetPlayerCharacter 0))
  (bind _returnvalue_2 (Game|GetPlayerController 0))
  (bind _asbp_player (Utilities|Casting|CastToBP_Player _returnvalue))
  (bind _springarm (Variables|/Game/Blueprints/BP_Player.BP_Player_C|GetSpringArm _asbp_player))
  ;[1 1 1] Comment
  (Components|Timeline|SetPlayRate (Variables|Default|GetWatch%20Pipe) (/ 1.0 (Variables|Default|GetTime_watch_Pipe)))
  (bind _rotation (Timeline|Watch%20Pipe Play)
    (:Update
      (Pawn|SetControlRotation _returnvalue_2 (Math|Rotator|Lerp(Rotator) (Pawn|GetControlRotation _returnvalue_2 :!class /Script/Engine.Controller) (Math|Rotator|Lerp(Rotator) (Transformation|GetWorldRotation _springarm) (Math|Rotator|FindLookatRotation (Transformation|GetWorldLocation _springarm) (Transformation|GetWorldLocation (Variables|/Game/Blueprints/Cinematics/BP_Pipes_Sound.BP_Pipes_Sound_C|GetCube (Variables|Default|GetPipes%20Sound%20Ref)))) _rotation true) _rotation true))
      (Input|DisableInput (.AsBP%20Player (Utilities|Casting|CastToBP_Player (Game|GetPlayerCharacter 0))) 0))
    (:Finished
      (Development|PrintString "DONEEEE"))))

(event Custom|Tilted%20Camera%20Ground
  (bind _returnvalue (Transformation|GetActorRotation))
  (bind (_roll _pitch _yaw) (Math|Rotator|BreakRotator _returnvalue))
  ;[1 1 1] Comment
  (Components|Timeline|SetPlayRate (Variables|Default|Gettilted%20camera) (/ 1.0 (Variables|Default|GetTilted%20Camera%20Rotation)))
  (bind _newtrack_0 (Timeline|Tilted%20Camera Play)
    (:Update
      (Pawn|SetControlRotation (Game|GetPlayerController 0) (Math|Rotator|Lerp(Rotator) (Variables|Default|GetHead's%20Up) (Math|Rotator|MakeRotator (- _roll 315.0) _pitch (- _yaw 3.6e+02)) _newtrack_0 true)))))

(event Custom|Lock%20look
  ;[1 1 1] Comment
  (bind _asbp_player (Utilities|Casting|CastToBP_Player (Game|GetPlayerCharacter 0)))
  (Variables|Default|GetPipes%20Sound%20Ref
    (:then
      (Pawn|SetControlRotation (Game|GetPlayerController 0) (Math|Rotator|FindLookatRotation (Transformation|GetWorldLocation (Variables|/Game/Blueprints/BP_Player.BP_Player_C|GetSpringArm _asbp_player)) (Transformation|GetWorldLocation (Variables|/Game/Blueprints/Cinematics/BP_Pipes_Sound.BP_Pipes_Sound_C|GetCube (Variables|Default|GetPipes%20Sound%20Ref))))))
    (:else)))

(event Custom|Lose%20Item%20In%20Hand
  ;[1 1 1] Comment
  (Default|Release (.AsBP%20Player (Utilities|Casting|CastToBP_Player (Game|GetPlayerCharacter 0)))))

(event EventBeginPlay
  ;[1 1 1] Comment
  (Actor|Tick|SetActorTickEnabled false)
  (Variables|Default|SetCurrent%20Rotation (Transformation|GetActorRotation))
  (Variables|Default|SetOriginal%20Target%20Offset (Variables|/Script/Engine.SpringArmComponent|GetTargetOffset (Variables|/Game/Blueprints/BP_Player.BP_Player_C|GetSpringArm (.AsBP%20Player (Utilities|Casting|CastToBP_Player (Game|GetPlayerCharacter 0)))))))

(event EventTick
  (params (DeltaSeconds :type Float%20%28single-precision%29))
  ;[1 1 1] Comment
  (if (Variables|Default|GetGrippedd)
    (CallFunction|LockLook)))

(fn ConstructionScript)