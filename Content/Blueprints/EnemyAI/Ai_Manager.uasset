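; AI manager for a monster enemy that picks the vent nearest the player when it senses a stimulus.
; On BeginPlay it hides the monster, teleports its capsule to the world origin, deactivates it and caches the player.
; Successful perception stores the noise location, then measures each vent's distance to the player rather than to the noise.
; The closest vent is saved and its name printed; the monster is not spawned or moved there.
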(event OnTargetPerceptionUpdated(AIPerception)
  (params (Actor :type Actor%20Object%20Reference) (Stimulus :type AI%20Stimulus%20Structure))
  (bind (_stimuluslocation _bsuccessfullysensed) (Utilities|Struct|BreakAIStimulus Stimulus))
  (if _bsuccessfullysensed
    (Variables|Default|SetNoise%20Location _stimuluslocation)
    (CallFunction|FindNearVent)))

(event Custom|Find_Near_Vent
  (for _array_element (Variables|Default|GetVents)
    (Variables|/Game/Blueprints/EnemyAI/BP_Vents.BP_Vents_C|SetDistanceWithPlayer _array_element (Math|Vector|Distance(Vector) (Transformation|GetWorldLocation (Variables|/Game/Blueprints/EnemyAI/BP_Vents.BP_Vents_C|GetDefaultSceneRoot _array_element)) (Transformation|GetWorldLocation (Variables|/Script/Engine.Character|GetCapsuleComponent (Variables|Default|GetPlayer_Ref))))))
  (for (_array_element_2 _array_index) (Variables|Default|GetVents)
    (if (not (== _array_index 0))
      (if (< (Variables|/Game/Blueprints/EnemyAI/BP_Vents.BP_Vents_C|GetDistanceWithPlayer _array_element_2) (Variables|/Game/Blueprints/EnemyAI/BP_Vents.BP_Vents_C|GetDistanceWithPlayer (Variables|Default|GetNear_Vent)))
        (Variables|Default|SetNear_Vent _array_element_2))
      (else
        (Variables|Default|SetNear_Vent _array_element_2))))
  (Development|PrintString (Utilities|GetDisplayName (Variables|Default|GetNear_Vent))))

(event EventBeginPlay
  (bind _monstre_ref (Variables|Default|GetMonstre_Ref))
  (Utilities|FlowControl|Sequence
    (:then_0
      (Rendering|SetVisibility (Variables|/Game/Blueprints/EnemyAI/BP_MonstreAI.BP_MonstreAI_C|GetStaticMesh _monstre_ref) false false)
      (Transformation|SetWorldLocation (Variables|/Script/Engine.Character|GetCapsuleComponent _monstre_ref) "0, 0, 0" false true)
      (Variables|/Game/Blueprints/EnemyAI/BP_MonstreAI.BP_MonstreAI_C|SetActivate? _monstre_ref false))
    (:then_1
      (bind _asbp_player (Utilities|Casting|CastToBP_Player (Game|GetPlayerCharacter 0)))
      (Variables|Default|SetPlayer_Ref _asbp_player))))

(fn ConstructionScript)