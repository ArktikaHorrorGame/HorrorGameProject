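; MainGameInstance is a game instance Blueprint that relocates the player start to a checkpoint.
; When the referenced CheckpointResetLevel has ResetLevel set, ChangePlayerStart moves the first PlayerStart found to that checkpoint's arrow location and rotation, gated by a DoOnce.
; GetGuardPost, GetNoiseLocation and GetPatrolPoints are stubs that return zero vectors or nothing.
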(event Custom|Change%20Player%20Start
  (bind _checkpoint_resetlevel (Variables|Default|GetCheckpoint_ResetLevel))
  (bind _arrow (Variables|/Game/Blueprints/BP_Object/BP_Checkpoint_ResetLevel.BP_Checkpoint_ResetLevel_C|GetArrow _checkpoint_resetlevel))
  (bind _returnvalue (Transformation|GetWorldTransform _arrow))
  (if (Variables|/Game/Blueprints/BP_Object/BP_Checkpoint_ResetLevel.BP_Checkpoint_ResetLevel_C|GetReset%20Level%20? (Variables|Default|GetCheckpoint_ResetLevel))
    (Utilities|FlowControl|DoOnce false
      (:Completed
        (bind _returnvalue_2 (Actor|GetActorOfClass "/Script/Engine.PlayerStart"))
        (Transformation|SetWorldLocationAndRotation (Variables|/Script/Engine.Actor|GetRootComponent _returnvalue_2) (.location _returnvalue) (.rotation _returnvalue) false false)))))

(fn GetGuardPost
  (return "0, 0, 0"))

(fn GetNoiseLocation
  (return "0, 0, 0"))

(fn GetPatrolPoints
  (return 0))