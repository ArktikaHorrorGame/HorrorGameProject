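; Patrol point manager that numbers every BP_PatrolPoint in the level within its patrol path for enemy AI.
; The same pass runs in the Construction Script and on BeginPlay, clearing Refresh and numbering points in GetAllActorsOfClass order.
; A struct array indexed by path caches each last order index, so numbering resumes when paths interleave.
; IncreaseOrderIndex sets each point's OrderIndex and text label, then updates that cache.
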(event Custom|Increase%20Order%20Index
  (params (Patrol%20Point :type BP%20Patrol%20Point%20Object%20Reference))
  (bind _current_patrol_path_index (Variables|Default|GetCurrent%20Patrol%20Path%20Index))
  (bind _result (Math|Integer|IncrementInt (Variables|Default|GetCache%20Order%20Index))
    (:%20%20
      (bind _output_get (Variables|/Game/Blueprints/EnemyAI/BP_PatrolPoint.BP_PatrolPoint_C|SetOrder%20Index Patrol%20Point _result))
      (Rendering|Components|TextRender|SetText (Variables|/Game/Blueprints/EnemyAI/BP_PatrolPoint.BP_PatrolPoint_C|GetOrder%20Text Patrol%20Point) (Utilities|Text|FormatText "Order: {Order}" _output_get))
      (Utilities|Array|SetArrayElem (Variables|Default|GetCache%20Order%20Index%20Struct) _current_patrol_path_index (Utilities|Struct|MakeS_PatrolPath _current_patrol_path_index _result)))))

(event EventBeginPlay
  (bind _cache_order_index_struct (Variables|Default|GetCache%20Order%20Index%20Struct))
  (Variables|Default|SetRefresh false)
  (bind _outactors (Actor|GetAllActorsOfClass "/Game/Blueprints/EnemyAI/BP_PatrolPoint.BP_PatrolPoint_C"))
  ;[1 1 1] Update the order index for the correct path
  (for _array_element _outactors
    (if (== (Variables|/Game/Blueprints/EnemyAI/BP_PatrolPoint.BP_PatrolPoint_C|GetPatrol%20Path%20Index _array_element) (Variables|Default|GetCurrent%20Patrol%20Path%20Index))
      (CallFunction|IncreaseOrderIndex _array_element)
      (else
        ;[1 1 1] Store the cache order index for each path (This is so that if the loop switches paths before finishing, it can continue where it left off when going back to that path
        (bind _output_get (Variables|Default|SetCurrent%20Patrol%20Path%20Index (Variables|/Game/Blueprints/EnemyAI/BP_PatrolPoint.BP_PatrolPoint_C|GetPatrol%20Path%20Index _array_element)))
        (if (Utilities|Array|IsValidIndex _cache_order_index_struct _output_get)
          (Variables|Default|SetCache%20Order%20Index (.CacheOrderIndex (Utilities|Struct|BreakS_PatrolPath (Utilities|Array|Get(acopy) _cache_order_index_struct _output_get))))
          (else
            (Utilities|Array|Add (Variables|Default|GetCache%20Order%20Index%20Struct) (Utilities|Struct|MakeS_PatrolPath (Variables|Default|GetCurrent%20Patrol%20Path%20Index) -1))
            (Variables|Default|SetCache%20Order%20Index -1)))
        (CallFunction|IncreaseOrderIndex _array_element)))))

(fn ConstructionScript
  (bind _cache_order_index_struct (Variables|Default|GetCache%20Order%20Index%20Struct))
  (Variables|Default|SetRefresh false)
  (bind _outactors (Actor|GetAllActorsOfClass "/Game/Blueprints/EnemyAI/BP_PatrolPoint.BP_PatrolPoint_C"))
  ;[1 1 1] Update the order index for the correct path
  (for _array_element _outactors
    (if (== (Variables|/Game/Blueprints/EnemyAI/BP_PatrolPoint.BP_PatrolPoint_C|GetPatrol%20Path%20Index _array_element) (Variables|Default|GetCurrent%20Patrol%20Path%20Index))
      (CallFunction|IncreaseOrderIndex _array_element)
      (else
        ;[1 1 1] Store the cache order index for each path (This is so that if the loop switches paths before finishing, it can continue where it left off when going back to that path
        (bind _output_get (Variables|Default|SetCurrent%20Patrol%20Path%20Index (Variables|/Game/Blueprints/EnemyAI/BP_PatrolPoint.BP_PatrolPoint_C|GetPatrol%20Path%20Index _array_element)))
        (if (Utilities|Array|IsValidIndex _cache_order_index_struct _output_get)
          (Variables|Default|SetCache%20Order%20Index (.CacheOrderIndex (Utilities|Struct|BreakS_PatrolPath (Utilities|Array|Get(acopy) _cache_order_index_struct _output_get))))
          (else
            (Utilities|Array|Add (Variables|Default|GetCache%20Order%20Index%20Struct) (Utilities|Struct|MakeS_PatrolPath (Variables|Default|GetCurrent%20Patrol%20Path%20Index) -1))
            (Variables|Default|SetCache%20Order%20Index -1)))
        (CallFunction|IncreaseOrderIndex _array_element)))))