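; Monster enemy that patrols, guards or searches by running a behavior tree per mode, switchable by events.
; When active, pawn sensing fills a reversible timeline meter (or detects instantly) to start a faster chase with music, ending after a retriggerable delay without sightings.
; Perceived noises set blackboard investigation unless chasing.
; Touching the player shows a widget and reloads the level; a vent return teleports to hard-coded coordinates.
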(event OnSeePawn(PawnSensing)
  (params (Pawn :type Pawn%20Object%20Reference))
  (bind _returnvalue (Utilities|Name|MakeLiteralName "CanSeePlayer?"))
  (bind _charactermovement (Variables|Character|GetCharacterMovement))
  (bind _ai_controller_ref (Variables|Default|GetAI%20Controller%20REF))
  (bind _returnvalue_2 (AI|GetBlackboard _ai_controller_ref))
  ;[1 1 1] Detect player
  (if (Variables|Default|GetActivate?)
    (if (== Pawn (Game|GetPlayerCharacter 0))
      (Utilities|FlowControl|Sequence
        (:then_0
          ;;[1 1 1] Fill up/drain detection meter
          (if (Variables|Default|GetDetect%20Immediately)
            (if (Variables|Default|GetIsInvestaging?) :!label _label
              (AI|Navigation|StopMovement (Variables|Default|GetAI%20Controller%20REF))
              (CallFunction|EndInvestigation)
              (Variables|Default|SetIsInvestaging? false))
            ;;[1 1 1] Start chasing
            (AI|Components|Blackboard|SetValueasBool _returnvalue_2 _returnvalue true)
            (Variables|/Script/Engine.CharacterMovementComponent|SetMaxWalkSpeed _charactermovement 4e+02)
            (Variables|Default|SetIsChasing? true)
            (Development|PrintString "see pleyer")
            (Utilities|FlowControl|DoOnce false :!label _label_2
              (:Completed
                (Audio|PlaySoundatLocation "/Game/Blueprints/Audio/SFX_Arthur/monstre/wav/monstre_-_cri_1.monstre_-_cri_1" (Transformation|GetActorLocation) "0, 0, 0" 1.0 1.0 0.0 0 0 0 0)
                (Class|BPIStealthAI|StartChaseMusic(Message) (Game|GetGameInstance))))
            (else
              (Utilities|FlowControl|Sequence
                (:then_0
                  (bind _direction (Timeline|Fill%20Detection%20Meter Play)
                    (:Finished
                      (switch Utilities|FlowControl|Switch|SwitchonETimelineDirection _direction
                        (:Forward
                          (goto _label))
                        (:Backward
                          ;;[1 1 1] Stop chasing
                          (AI|Components|Blackboard|SetValueasBool _returnvalue_2 _returnvalue false :!label _label_3)
                          (Variables|/Script/Engine.CharacterMovementComponent|SetMaxWalkSpeed _charactermovement 1.5e+02)
                          (Variables|Default|SetIsChasing? false)
                          (Class|BPIStealthAI|StopChaseMusic(Message) (Game|GetGameInstance))
                          (goto _label_2 Reset))))))
                (:then_1
                  (Utilities|FlowControl|DoOnce false :!label _label_4
                    (:Completed
                      (Audio|PlaySoundatLocation "/Game/Blueprints/Audio/SFX_Arthur/monstre/wav/monstre-respiration-2.monstre-respiration-2" (Transformation|GetActorLocation) "0, 0, 0" 1.0 1.0 0.0 0 0 0 0))))))))
        (:then_1
          (Utilities|FlowControl|RetriggerableDelay (Variables|Search|GetSearch%20Time))
          (if (Variables|Default|GetDetect%20Immediately)
            (goto _label_3)
            (else
              (Audio|Components|Audio|Stop (Variables|Default|GetFill%20Detection%20Meter))
              (Utilities|FlowControl|Sequence
                (:then_0
                  (goto _label_4 Reset))
                (:then_1
                  (Timeline|Fill%20Detection%20Meter Reverse))))))))))

(event OnComponentBeginOverlap(Trigger_Death)
  (params (OverlappedComponent :type Primitive%20Component%20Object%20Reference) (OtherActor :type Actor%20Object%20Reference) (OtherComp :type Primitive%20Component%20Object%20Reference) (OtherBodyIndex :type Integer) (bFromSweep :type Boolean) (SweepResult :type Hit%20Result%20Structure%20%28by%20ref%29))
  (Utilities|Casting|CastToBP_Player OtherActor)
  (bind _returnvalue (UserInterface|CreateWidget "/Game/Blueprints/gif/CoincoinW.CoincoinW_C" (Game|GetPlayerController 0)))
  (UserInterface|Viewport|AddtoViewport _returnvalue 0)
  (Utilities|Time|SetTimerbyEvent (delegate Custom|Restart_Level) 3.0))

(event OnTargetPerceptionUpdated(AIPerception)
  (params (Actor :type Actor%20Object%20Reference) (Stimulus :type AI%20Stimulus%20Structure))
  (bind (_age _expirationage _strength _stimuluslocation _receiverlocation _tag _bsuccessfullysensed) (Utilities|Struct|BreakAIStimulus Stimulus))
  ;[1 1 1] Investigate any noise heard
  (if (Variables|Default|GetActivate?)
    (if _bsuccessfullysensed
      (Variables|Default|SetNoise%20Location _stimuluslocation)
      (if (not (Variables|Default|GetIsChasing?))
        (if (not (Variables|Default|GetIsInvestaging?))
          (Variables|Default|SetIsInvestaging? true)
          (else
            (AI|Navigation|StopMovement (Variables|Default|GetAI%20Controller%20REF))))
        (AI|Components|Blackboard|SetValueasBool (AI|GetBlackboard (Variables|Default|GetAI%20Controller%20REF)) (Utilities|Name|MakeLiteralName "HeardNoise?") true)
        (if (Variables|Default|GetTimerRespiration)
          (bind _returnvalue (Utilities|Time|SetTimerbyEvent (delegate Custom|Respiration) 5.0))
          (Variables|Default|SetTimer%20Respiration _returnvalue)
          ;;[1 1 1] Sound when he heard a Noise
          (Audio|PlaySoundatLocation "/Game/Blueprints/Audio/SFX_Arthur/monstre/wav/monstre-respiration-1.monstre-respiration-1" (Transformation|GetActorLocation) "0, 0, 0" 1.0 1.0 0.0 0 0 0 0)
          (Variables|Default|SetTimerRespiration false))))))

(event Custom|Respiration
  ;[1 1 1] Investigate any noise heard
  (Variables|Default|SetTimerRespiration true)
  (Utilities|Time|ClearandInvalidateTimerbyHandle (Variables|Default|GetTimer%20Respiration)))

(event Custom|Restart_Level
  (Game|OpenLevel(byObjectReference) "/Game/Maps/BlockOutLDV1.BlockOutLDV1"))

(event Custom|ChangeToNull
  ;[1 1 1] Change Behavior
  (AI|RunBehaviorTree (Variables|Default|GetAI%20Controller%20REF) "/Game/Blueprints/EnemyAI/BT/BT_SAI_Null.BT_SAI_Null")
  (Variables|Default|SetActivate? false))

(event Custom|ChangeToSearch
  ;[1 1 1] Change Behavior
  (AI|RunBehaviorTree (Variables|Default|GetAI%20Controller%20REF) "/Game/Blueprints/EnemyAI/BT/BT_SAI_Search.BT_SAI_Search")
  (if (not (Variables|Default|GetActivate?))
    (Variables|Default|SetActivate? true)))

(event Custom|Go_back_to_vent
  (if (Variables|Default|GetReturnVent?)
    (Development|PrintString "Hello" true true "(R=1.000000,G=0.000000,B=0.023868,A=1.000000)")
    (if (Variables|Default|GetIs_at_guard_post)
      ;[1 1 1] Anim_return_vent
      (Animation|PlayAnimMontage 0 1.0 "None")
      ;[1 1 1] Retour son spawn (il faudrait la changer quand on aura fini la map)
      (Transformation|SetWorldLocation (Variables|Collision|GetCapsuleComponent) (Math|Vector|MakeVector -2.7e+03 -9e+02 188.0) false true)
      (Variables|Default|SetReturnVent? false))))

(event Custom|ChangeToPatrol
  (params (IndexPatrol :type Integer))
  ;[1 1 1] Change Behavior
  (Variables|PatrolPoints|SetPatrol%20Path%20Index IndexPatrol)
  (AI|RunBehaviorTree (Variables|Default|GetAI%20Controller%20REF) "/Game/Blueprints/EnemyAI/BT/BT_SAI_Patrol.BT_SAI_Patrol")
  (if (not (Variables|Default|GetActivate?))
    (Variables|Default|SetActivate? true)))

(event Custom|ChangeToGuard
  ;[1 1 1] Change Behavior
  (AI|RunBehaviorTree (Variables|Default|GetAI%20Controller%20REF) "/Game/Blueprints/EnemyAI/BT/BT_SAI_Guard.BT_SAI_Guard")
  (if (not (Variables|Default|GetActivate?))
    (Variables|Default|SetActivate? true)))

(event EventBeginPlay
  (Utilities|FlowControl|Sequence
    (:then_0
      ;[1 1 1] Set AI type
      (Variables|Default|SetAI%20Controller%20REF (AI|GetAIController self))
      (switch Utilities|FlowControl|Switch|SwitchonE_AI_Type (Variables|Default|GetAI%20Type)
        (:NewEnumerator0
          (AI|RunBehaviorTree (Variables|Default|GetAI%20Controller%20REF) "/Game/Blueprints/EnemyAI/BT/BT_SAI_Search.BT_SAI_Search"))
        (:NewEnumerator1
          (AI|RunBehaviorTree (Variables|Default|GetAI%20Controller%20REF) "/Game/Blueprints/EnemyAI/BT/BT_SAI_Patrol.BT_SAI_Patrol"))
        (:NewEnumerator2
          (AI|RunBehaviorTree (Variables|Default|GetAI%20Controller%20REF) "/Game/Blueprints/EnemyAI/BT/BT_SAI_Guard.BT_SAI_Guard"))
        (:NewEnumerator3
          (AI|RunBehaviorTree (Variables|Default|GetAI%20Controller%20REF) "/Game/Blueprints/EnemyAI/BT/BT_SAI_Null.BT_SAI_Null"))))
    (:then_1
      ;[1 1 1] Set guard post position
      (Variables|GuardPost|SetGuardPostPosition (Math|Vector|SelectVector (Transformation|GetActorLocation) (Variables|GuardPost|GetGuardPostPosition) (Variables|GuardPost|GetUse%20Current%20Position?))))
    (:then_2
      ;[1 1 1] Set the detection time
      (Components|Timeline|SetPlayRate (Variables|Default|GetFill%20Detection%20Meter) (/ 1.0 (Variables|Default|GetDetection%20Time))))))

(event EventEndInvestigation
  ;[1 1 1] Investigate any noise heard
  (AI|Components|Blackboard|SetValueasBool (AI|GetBlackboard (Variables|Default|GetAI%20Controller%20REF)) (Utilities|Name|MakeLiteralName "HeardNoise?") false))

(fn ConstructionScript)

(fn GetGuardPost
  (return (Variables|GuardPost|GetGuardPostPosition)))

(fn GetNoiseLocation
  (return (Variables|Default|GetNoise%20Location)))

(fn GetpatrolPoints
  ;[1 1 1] Get the patrol points on the desired patrol path
  (bind _outactors (Actor|GetAllActorsOfClass "/Game/Blueprints/EnemyAI/BP_PatrolPoint.BP_PatrolPoint_C"))
  (for _array_element _outactors
    (if (== (Variables|/Game/Blueprints/EnemyAI/BP_PatrolPoint.BP_PatrolPoint_C|GetPatrol%20Path%20Index _array_element) (Variables|PatrolPoints|GetPatrol%20Path%20Index))
      (Utilities|Array|Add (Variables|Default|GetPatrol%20Path) _array_element)))
  (return (Variables|Default|GetPatrol%20Path)))