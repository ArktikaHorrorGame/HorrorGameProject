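; Fuse box actor that shows inserted fuses and enables a freight lift (MonteCharge) once two are in place.
; Its Interaction event switches on NbrFusible, revealing one fuse mesh at one and both at two.
; At two it also sets FusibleBon on the referenced lift and spawns spark emitters at placed marker components.
; The count is only read here, never changed.
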(event EventInteraction
  (bind _p_sparks_c3 (Variables|Default|GetP_Sparks_C3))
  (bind _p_sparks_c4 (Variables|Default|GetP_Sparks_C4))
  (bind _p_sparks_c5 (Variables|Default|GetP_Sparks_C5))
  (bind _p_sparks_c6 (Variables|Default|GetP_Sparks_C6))
  (bind _p_sparks_c1 (Variables|Default|GetP_Sparks_C1))
  (bind _p_sparks_c2 (Variables|Default|GetP_Sparks_C2))
  (bind _returnvalue (Transformation|GetWorldTransform _p_sparks_c2))
  (bind _returnvalue_2 (Transformation|GetWorldTransform _p_sparks_c3))
  (bind _returnvalue_3 (Transformation|GetWorldTransform _p_sparks_c4))
  (bind _returnvalue_4 (Transformation|GetWorldTransform _p_sparks_c5))
  (bind _returnvalue_5 (Transformation|GetWorldTransform _p_sparks_c6))
  (bind _returnvalue_6 (Transformation|GetWorldTransform _p_sparks_c1))
  (switch int (Variables|Default|GetNbr_Fusible)
    (:1
      (Development|SetHiddeninGame (Variables|Default|GetFusible) false false))
    (:2
      (Development|SetHiddeninGame (Variables|Default|GetFusible2) false false)
      (Development|SetHiddeninGame (Variables|Default|GetFusible) false false)
      (Variables|/Game/Blueprints/Bp_Monte_Charge.Bp_Monte_Charge_C|SetFusible_Bon? (Variables|Default|GetMonteCharge_Ref) true)
      (Effects|SpawnEmitteratLocation "/Game/Blueprints/VFX_Manu/Particles/Sparks/P_Sparks_C.P_Sparks_C" (.location _returnvalue_6) (.rotation _returnvalue_6) (.scale _returnvalue_6))
      (Effects|SpawnEmitteratLocation "/Game/Blueprints/VFX_Manu/Particles/Sparks/P_Sparks_E.P_Sparks_E" (.location _returnvalue) (.rotation _returnvalue) (.scale _returnvalue))
      (Effects|SpawnEmitteratLocation "/Game/Blueprints/VFX_Manu/Particles/Sparks/P_Sparks_C.P_Sparks_C" (.location _returnvalue_2) (.rotation _returnvalue_2) (.scale _returnvalue_2))
      (Effects|SpawnEmitteratLocation "/Game/Blueprints/VFX_Manu/Particles/Sparks/P_Sparks_E.P_Sparks_E" (.location _returnvalue_3) (.rotation _returnvalue_3) (.scale _returnvalue_3))
      (Effects|SpawnEmitteratLocation "/Game/Blueprints/VFX_Manu/Particles/Sparks/P_Sparks_E.P_Sparks_E" (.location _returnvalue_4) (.rotation _returnvalue_4) (.scale _returnvalue_4))
      (Effects|SpawnEmitteratLocation "/Game/Blueprints/VFX_Manu/Particles/Sparks/P_Sparks_E.P_Sparks_E" (.location _returnvalue_5) (.rotation _returnvalue_5) (.scale _returnvalue_5)))))

(fn ConstructionScript)