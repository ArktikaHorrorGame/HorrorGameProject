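; Physics-hinged door, grabbed through Pickup/Drop, that can require a key and an unlocked valve wheel (child BP_Wheel linked back to the door).
; Pickup frees the hinge constraint and plays locked feedback, or clears the key's HUD slot and reveals the wheel.
; A successful grab glides the player to a front or rear anchor chosen by view angle.
; Hits from the player or BP_Fix_Grab_Leget re-lock the hinge swing.
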(event OnComponentHit(MainMesh)
  (params (HitComponent :type Primitive%20Component%20Object%20Reference) (OtherActor :type Actor%20Object%20Reference) (OtherComp :type Primitive%20Component%20Object%20Reference) (NormalImpulse :type Vector :default "0, 0, 0") (Hit :type Hit%20Result%20Structure%20%28by%20ref%29))
  (bind _locker (Variables|Default|GetLocker))
  (Utilities|Casting|CastToBP_Player OtherActor
    (:then
      _)
    (:CastFailed
      (Utilities|Casting|CastToBP_Fix_Grab_Leget OtherActor)))
  (Class|PhysicsConstraintComponent|SetConstrainedComponents _locker (Variables|Default|GetMainMesh) "None" (Variables|Default|GetRoot) "None")
  (Class|PhysicsConstraintComponent|SetAngularSwing1Limit _locker "ACM_Locked" 0.0))

(event Custom|Verify_Behind/InFront
  (bind _returnvalue (Transformation|GetActorLocation))
  (bind _returnvalue_2 (Game|GetPlayerController 0))
  (bind (_location _rotation) (Pawn|GetPlayerViewPoint _returnvalue_2))
  (bind _returnvalue_3 (- _returnvalue _location))
  (bind _returnvalue_4 (Math|Vector|Normalize _returnvalue_3))
  (if (< (Class|KismetMathLibrary|DegAtan2 (Math|Vector|DotProduct _returnvalue_4 (Math|Vector|Normalize (Math|Vector|GetRightVector _rotation))) (Math|Vector|DotProduct _returnvalue_4 (Math|Vector|Normalize (Math|Vector|GetForwardVector _rotation)))) -1.0)
    (Variables|Default|SetD_Player_T (Transformation|GetWorldTransform (Variables|Default|GetD_Player_Arriere)))
    (else
      (Variables|Default|SetD_Player_T (Transformation|GetWorldTransform (Variables|Default|GetD_Player_Avant))))))

(event Custom|Delete_Widget
  (Class|Image|SetOpacity (Variables|/Game/Blueprints/Widget/Inventory.Inventory_C|GetSlot1 (Variables|/Game/Blueprints/BP_Player.BP_Player_C|GetHud_Inventory (Variables|Default|GetPlayer_Ref))) 0.0))

(event Custom|Anim_Locked
  (Physics|SetSimulatePhysics (Variables|Default|GetMainMesh) false)
  (bind _alpha (Timeline|Timeline_0 PlayFromStart)
    (:Update
      (Transformation|SetRelativeRotation (Variables|Default|GetMainMesh) (Math|Rotator|Lerp(Rotator) "0, 0, 0" "0.000000,1.000000,0.000000" _alpha true) false false))
    (:Finished
      (Physics|SetSimulatePhysics (Variables|Default|GetMainMesh) true))))

(event EventBeginPlay
  (|CallParentFunction)
  (Variables|Default|SetPlayer_Ref (.AsBP%20Player (Utilities|Casting|CastToBP_Player (Game|GetPlayerCharacter 0))))
  (Components|Timeline|SetPlayRate (Variables|Default|GetTimeline) (/ 1.0 (Variables|Default|GetTime_Deplacement_Door)))
  (Rendering|SetVisibility (Variables|/Game/Blueprints/BP_Object/BP_BaseObject.BP_BaseObject_C|GetMainMesh (.AsBP%20Wheel (Utilities|Casting|CastToBP_Wheel (Variables|/Script/Engine.ChildActorComponent|GetChildActor (Variables|Default|GetBP_Wheel))))) false false))

(event Collision|EventActorBeginOverlap
  (params (OtherActor :type Actor%20Object%20Reference)))

(event EventPickup
  (params (Hit :type Hit%20Result%20Structure))
  (bind _returnvalue (Transformation|GetActorLocation))
  (bind _d_player_t (Variables|Default|GetD_Player_T))
  (Class|PhysicsConstraintComponent|SetAngularSwing1Limit (Variables|Default|GetLocker) "ACM_Free" 0.0)
  (if (Variables|Default|GetNeed%20Key%20?)
    (if (Variables|Default|GetHas%20Key%20?)
      (CallFunction|DeleteWidget)
      (if (Variables|Default|GetHas_Valve)
        (Rendering|SetVisibility (Variables|/Game/Blueprints/BP_Object/BP_BaseObject.BP_BaseObject_C|GetMainMesh (.AsBP%20Wheel (Utilities|Casting|CastToBP_Wheel (Variables|/Script/Engine.ChildActorComponent|GetChildActor (Variables|Default|GetBP_Wheel))))) true false)
        (if (Variables|Default|GetValveUnlock)
          (Utilities|FlowControl|Sequence :!label _label
            (:then_0
              (Utilities|FlowControl|DoOnce false
                (:Completed
                  (Audio|PlaySoundatLocation "/Game/Blueprints/Audio/SFX_Final/Key/Key_Unlock.Key_Unlock" _returnvalue "0, 0, 0" 1.0 1.0 0.0 0 0 0 0))))
            (:then_1
              (|CallParentFunction Hit :!label _label_2)
              (CallFunction|VerifyBehind/InFront)
              (bind _output_get (Variables|Default|SetPlayer_T (Transformation|GetActorTransform (Variables|Default|GetPlayer_Ref))))
              (Components|Timeline|SetNewTime (Variables|Default|GetTimeline) 0.0)
              (bind _alpha_move (Timeline|Timeline Play)
                (:Update
                  (Transformation|SetActorTransform (Variables|Default|GetPlayer_Ref) (Math|Transform|Lerp(Transform) (Variables|Default|GetPlayer_T) (Math|Transform|MakeTransform (Math|Vector|MakeVector (.x (.location _d_player_t)) (.y (.location _d_player_t)) (.z (.location _output_get))) (.rotation _d_player_t) (.scale _output_get)) _alpha_move)))))))
        (else
          (goto _label)))
      (else
        (Audio|PlaySoundatLocation "/Game/Blueprints/Audio/SFX_Final/Key/Key_Locked.Key_Locked" _returnvalue "0, 0, 0" 1.0 1.0 0.0 0 0 0 0)
        (if (Variables|Default|GetDo_Anim_Lock)
          (CallFunction|AnimLocked))))
    (else
      (Variables|Default|SetHas%20Key%20? true)
      (goto _label_2))))

(event EventDrop
  (|CallParentFunction)
  (Audio|Components|Audio|Stop (Variables|Default|GetTimeline)))

(fn ConstructionScript
  (|CallParentFunction)
  (Variables|/Game/Blueprints/BP_Object/BP_Wheel.BP_Wheel_C|SetLinkedActor (.AsBP%20Wheel (Utilities|Casting|CastToBP_Wheel (Variables|/Script/Engine.ChildActorComponent|GetChildActor (Variables|Default|GetBP_Wheel)))) self))