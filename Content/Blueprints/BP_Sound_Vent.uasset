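; BP_Sound_Vent is an actor that moves a sound along a spline, by its name a vent sound, then destroys itself.
; On BeginPlay it sets the playback rate from the inverse of TimePlayRate and starts a timeline.
; The timeline's track lerps distance from zero to the last spline point, placing the Audio component at that world location each update.
; When the timeline finishes, the actor is destroyed.
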(event Custom|Follow%20Spline
  (bind _spline (Variables|Default|GetSpline))
  (bind _newtrack_0 (Timeline|Spline_Sound Play)
    (:Update
      (Transformation|SetWorldLocation (Variables|Default|GetAudio) (Spline|GetLocationatDistanceAlongSpline _spline (Math|Float|Lerp 0.0 (Spline|GetDistanceAlongSplineatSplinePoint _spline (- (Spline|GetNumberOfSplinePoints _spline) 1)) _newtrack_0) "World") false false))
    (:Finished
      (Actor|DestroyActor))))

(event EventBeginPlay
  (Components|Timeline|SetPlayRate (Variables|Default|GetSpline_Sound) (/ 1.0 (Variables|Default|GetTime/PlayRate)))
  (CallFunction|FollowSpline))

(fn ConstructionScript)