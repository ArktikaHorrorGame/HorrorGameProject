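; BP_Fusible is a fuse pickup that the player collects through an Interaction event.
; Interaction plays a pickup sound and increments the fuse count on the referenced fuse box (BoiteFusibleRef).
; At a count of one or two, it sets Fuse1 or Fuse2 respectively and destroys itself.
; A sphere overlap toggles the mesh's Highlight material parameter while something is in range.
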(event OnComponentBeginOverlap(Sphere)
  (params (OverlappedComponent :type Primitive%20Component%20Object%20Reference) (OtherActor :type Actor%20Object%20Reference) (OtherComp :type Primitive%20Component%20Object%20Reference) (OtherBodyIndex :type Integer) (bFromSweep :type Boolean) (SweepResult :type Hit%20Result%20Structure%20%28by%20ref%29))
  (Rendering|Material|SetScalarParameterValueonMaterials (Variables|Default|GetStaticMesh) "Highlight" 1.0))

(event OnComponentEndOverlap(Sphere)
  (params (OverlappedComponent :type Primitive%20Component%20Object%20Reference) (OtherActor :type Actor%20Object%20Reference) (OtherComp :type Primitive%20Component%20Object%20Reference) (OtherBodyIndex :type Integer))
  (Rendering|Material|SetScalarParameterValueonMaterials (Variables|Default|GetStaticMesh) "Highlight" 0.0))

(event EventInteraction
  (bind _boite_fusible_ref (Variables|Default|GetBoite_Fusible_Ref))
  (Audio|PlaySoundatLocation "/Game/Blueprints/Audio/SFX_Final/Machines/Fusible_Pickup.Fusible_Pickup" (Transformation|GetActorLocation) "0, 0, 0" 1.0 1.0 0.0 0 0 0 0)
  (Variables|/Game/Blueprints/BP_Boite_Fusible.BP_Boite_Fusible_C|SetNbr_Fusible _boite_fusible_ref (+ (Variables|/Game/Blueprints/BP_Boite_Fusible.BP_Boite_Fusible_C|GetNbr_Fusible _boite_fusible_ref) 1))
  (if (== (Variables|/Game/Blueprints/BP_Boite_Fusible.BP_Boite_Fusible_C|GetNbr_Fusible _boite_fusible_ref) 1)
    (Variables|Default|SetFuse1 true)
    (Actor|DestroyActor)
    (elif (== (Variables|/Game/Blueprints/BP_Boite_Fusible.BP_Boite_Fusible_C|GetNbr_Fusible _boite_fusible_ref) 2)
      (Variables|Default|SetFuse2 true)
      (Actor|DestroyActor))))

(fn ConstructionScript)