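; Physics-driven door Blueprint that can be grabbed and gives locked feedback.
; Grabbing enables physics simulation on the door and, if it is locked and not unlocking, plays a pitch-randomized sound at the grab location and calls the locked animation.
; A timeline drives that jiggle through a slight rotation lerp, with a leftover debug print.
; The physics constraint swing-limit setup is unconnected and never runs.
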(event Custom|Anim_Locked
  (bind _alpha (Timeline|Timeline PlayFromStart)
    (:Update
      (Transformation|SetRelativeRotation (Variables|Default|GetDoor) (Math|Rotator|Lerp(Rotator) "0, 0, 0" "0,1.000000, 0" _alpha true) false false)
      (Development|PrintString "Hello"))))

(event EventBeginPlay)

(event EventGrabDoor
  (params (GrabPoint_Location :type Scene%20Component%20Object%20Reference) (Cam%20/Camera%20Arm :type Camera%20Component%20Object%20Reference) (BP_Player_Ref :type BP%20Player%20Object%20Reference))
  (Physics|SetSimulatePhysics (Variables|Default|GetDoor) true)
  ;[0 0 0] play 'Locked Jiggle' timeline if object is locked
  (if (and (Variables|Default|GetLocked) (not (Variables|Default|GetUnlocking)))
    (Audio|SpawnSoundatLocation 0 (Variables|Default|GetGrab%20location) "0, 0, 0" (Variables|Default|GetVolume%20Locked%20Door) (Math|Random|RandomFloatinRange 0.9 1.0) 0.0 0 0)
    (CallFunction|AnimLocked)))

(fn ConstructionScript)