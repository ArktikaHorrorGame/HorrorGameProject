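; BP_Sortie_Vent_Piege is a vent trap that makes the referenced monster burst out when the object is activated.
; Activation fades in monster ambience, nulls the monster's state, starts a vent-exit montage and moves its capsule to the trap's scene location.
; When the montage completes, a selection value switches the monster into either chase or patrol.
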(event Custom|Activate_Monster
  (bind _monstre_ref (Variables|Default|GetMonstre_Ref))
  (switch int (Variables|Default|GetSelection)
    (:0
      (Default|ChangetoChasse _monstre_ref 1e+03))
    (:1
      (Default|ChangetoPatrol _monstre_ref 1))))

(event EventObjectActivate
  (bind _monstre_ref (Variables|Default|GetMonstre_Ref))
  (bind _music (Variables|Default|GetMusic))
  (bind _audiocomponent (Variables|/Script/Engine.AmbientSound|GetAudioComponent _music))
  (Audio|Components|Audio|SetSound _audiocomponent "/Game/Blueprints/Audio/SFX_Final/Monstre/Monster_Ambiance.Monster_Ambiance")
  (Audio|Components|Audio|FadeIn _audiocomponent 4.0 1.0 0.0 "Linear" :!class /Script/Engine.AudioComponent)
  (Default|ChangetoNull _monstre_ref)
  (Animation|Montage|PlayMontage (Variables|/Script/Engine.Character|GetMesh _monstre_ref) "/Game/Blueprints/Animation/Sortie_Vent_Rapide/Sortie_de_vent_rapide-Course_BON_Bake_Montage.Sortie_de_vent_rapide-Course_BON_Bake_Montage"
    (:then
      (Transformation|SetWorldLocation (Variables|/Script/Engine.Character|GetCapsuleComponent _monstre_ref) (Transformation|GetWorldLocation (Variables|Default|GetScene)) false false))
    (:OnCompleted
      (CallFunction|ActivateMonster))))

(fn ConstructionScript)