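; Freight elevator (monte-charge) that an interaction sends alternately up and down, provided its fuse flag FusibleBon is set.
; A FlipFlop plays or reverses a timeline that lerps the platform mesh between two marker components, with travel time set by TDeplacement.
; Each trip plays motor and button sounds and locks player movement until the timeline finishes.
; A sphere overlap toggles a material highlight on the Cube.
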(event OnComponentBeginOverlap(Sphere)
  (params (OverlappedComponent :type Primitive%20Component%20Object%20Reference) (OtherActor :type Actor%20Object%20Reference) (OtherComp :type Primitive%20Component%20Object%20Reference) (OtherBodyIndex :type Integer) (bFromSweep :type Boolean) (SweepResult :type Hit%20Result%20Structure%20%28by%20ref%29))
  (Rendering|Material|SetScalarParameterValueonMaterials (Variables|Default|GetCube) "Highlight" 1.0))

(event OnComponentEndOverlap(Sphere)
  (params (OverlappedComponent :type Primitive%20Component%20Object%20Reference) (OtherActor :type Actor%20Object%20Reference) (OtherComp :type Primitive%20Component%20Object%20Reference) (OtherBodyIndex :type Integer))
  (Rendering|Material|SetScalarParameterValueonMaterials (Variables|Default|GetCube) "Highlight" 0.0))

(event Custom|Elevate_elavator
  (bind _returnvalue (Transformation|GetActorLocation))
  (Audio|PlaySoundatLocation "/Game/Blueprints/Audio/SFX_Final/Machines/bruit_de_monte_charge_silencieux.bruit_de_monte_charge_silencieux" _returnvalue "0, 0, 0" 1.0 1.0 0.0 0 0 0 0)
  (Audio|PlaySoundatLocation "/Game/Blueprints/Audio/SFX_Final/Machines/bouton_qui_s_active.bouton_qui_s_active" _returnvalue "0, 0, 0" 1.0 1.0 0.0 0 0 0 0)
  (bind _elevator (Timeline|Timeline Play)
    (:Update
      (Transformation|SetWorldLocation (Variables|Default|GetStaticMesh1) (Math|Vector|Lerp(Vector) (Transformation|GetWorldLocation (Variables|Default|GetB_Monte_Charge)) (Transformation|GetWorldLocation (Variables|Default|GetH_Monte_Charge)) _elevator) false false))
    (:Finished
      (Variables|/Game/Blueprints/BP_Player.BP_Player_C|SetCan_Move? (.AsBP%20Player (Utilities|Casting|CastToBP_Player (Game|GetPlayerCharacter 0))) true))))

(event Custom|Reverse_elevator
  (bind _returnvalue (Transformation|GetActorLocation))
  (Audio|Components|Audio|Stop (Variables|Default|GetTimeline))
  (Audio|PlaySoundatLocation "/Game/Blueprints/Audio/SFX_Final/Machines/bruit_de_monte_charge_silencieux.bruit_de_monte_charge_silencieux" _returnvalue "0, 0, 0" 1.0 1.0 0.0 0 0 0 0)
  (Audio|PlaySoundatLocation "/Game/Blueprints/Audio/SFX_Final/Machines/bouton_qui_s_active.bouton_qui_s_active" _returnvalue "0, 0, 0" 1.0 1.0 0.0 0 0 0 0)
  (bind _elevator (Timeline|Timeline Reverse)
    (:Update
      (Transformation|SetWorldLocation (Variables|Default|GetStaticMesh1) (Math|Vector|Lerp(Vector) (Transformation|GetWorldLocation (Variables|Default|GetB_Monte_Charge)) (Transformation|GetWorldLocation (Variables|Default|GetH_Monte_Charge)) _elevator) false false))
    (:Finished
      (Variables|/Game/Blueprints/BP_Player.BP_Player_C|SetCan_Move? (.AsBP%20Player (Utilities|Casting|CastToBP_Player (Game|GetPlayerCharacter 0))) true))))

(event EventBeginPlay
  (Components|Timeline|SetPlayRate (Variables|Default|GetTimeline) (/ 1.0 (Variables|Default|GetT_Deplacement))))

(event EventInteraction
  (if (Variables|Default|GetFusible_Bon?)
    (Variables|/Game/Blueprints/BP_Player.BP_Player_C|SetCan_Move? (.AsBP%20Player (Utilities|Casting|CastToBP_Player (Game|GetPlayerCharacter 0))) false)
    (Utilities|FlowControl|FlipFlop
      (:A
        (CallFunction|ElevateElavator))
      (:B
        (CallFunction|ReverseElevator)))))

(fn ConstructionScript)