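; BP_Child_BrokenGlassTrap is a broken glass trap that makes noise and can alert the monster when the player steps into it.
; Its box overlap, filtered to BP_Player, plays a quiet sound at the trap's location every time.
; If IsActivate is set, it also calls ChangeToChasse on MonstreRef to switch the monster to chase.
; The construction script only runs the parent's.
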(event OnComponentBeginOverlap(Box)
  (params (OverlappedComponent :type Primitive%20Component%20Object%20Reference) (OtherActor :type Actor%20Object%20Reference) (OtherComp :type Primitive%20Component%20Object%20Reference) (OtherBodyIndex :type Integer) (bFromSweep :type Boolean) (SweepResult :type Hit%20Result%20Structure%20%28by%20ref%29))
  (Utilities|Casting|CastToBP_Player OtherActor)
  (Audio|PlaySoundatLocation (Variables|Default|GetSound) (Transformation|GetActorLocation) (Transformation|GetActorRotation) 0.2 1.0 0.0 0 0 0 0)
  (if (Variables|Default|GetIs_Activate?)
    (Default|ChangetoChasse (Variables|Default|GetMonstre_Ref) 1e+03)))

(fn ConstructionScript
  (|CallParentFunction))