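; Grabbable door that can require a key and, optionally, an unlocked valve wheel before opening.
; Successful pickup runs the parent grab, then a timeline slides the player to a front or back anchor chosen by view angle; dropping stops it.
; Without the key it plays a locked sound and optional rattle, briefly suspending mesh physics.
; Construction links the child BP_Wheel to the door and disables its mesh collision.
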(event Custom|Verify_Behind/InFront
  (bind _returnvalue (Transformation|GetActorLocation))
  (bind _returnvalue_2 (Game|GetPlayerController 0))
  (bind (_location _rotation) (Pawn|GetPlayerViewPoint _returnvalue_2))
  (bind _returnvalue_3 (- _returnvalue _location))
  (bind _returnvalue_4 (Math|Vector|Normalize _returnvalue_3))
  (if (< (Class|KismetMathLibrary|DegAtan2 (Math|Vector|DotProduct _returnvalue_4 (Math|Vector|Normalize (Math|Vector|GetRightVector _rotation))) (Math|Vector|DotProduct _returnvalue_4 (Math|Vector|Normalize (Math|Vector|GetForwardVector _rotation)))) -1.0)
    (Variables|Default|SetD_Player_T (Transformation|GetWorldTransform (Variables|Default|GetD_Player_Arriere)))
    (else
      (Variables|Default|SetD_Player_T (Transformation|GetWorldTransform (Variables|Default|GetD_Player_Avant))))))

(event Custom|Anim_Locked
  (Physics|SetSimulatePhysics (Variables|Default|GetMainMesh) false)
  (bind _alpha (Timeline|Timeline_0 PlayFromStart)
    (:Update
      (Transformation|SetRelativeRotation (Variables|Default|GetMainMesh) (Math|Rotator|Lerp(Rotator) "0, 0, 0" "0.000000,1.000000,0.000000" _alpha true) false false))
    (:Finished
      (Physics|SetSimulatePhysics (Variables|Default|GetMainMesh) true))))

(event EventBeginPlay
  (|CallParentFunction)
  (Variables|Default|SetPlayer_Ref (.AsBP%20Player (Utilities|Casting|CastToBP_Player (Game|GetPlayerCharacter 0))))
  (Components|Timeline|SetPlayRate (Variables|Default|GetTimeline) (/ 1.0 (Variables|Default|GetTime_Deplacement_Door))))

(event Collision|EventActorBeginOverlap
  (params (OtherActor :type Actor%20Object%20Reference)))

(event EventPickup
  (params (Hit :type Hit%20Result%20Structure))
  (bind _returnvalue (Transformation|GetActorLocation))
  (bind _d_player_t (Variables|Default|GetD_Player_T))
  (if (Variables|Default|GetNeed%20Key%20?)
    (if (Variables|Default|GetHas%20Key%20?)
      (if (Variables|Default|GetHas_Valve)
        (if (Variables|Default|GetValveUnlock)
          (Utilities|FlowControl|Sequence :!label _label
            (:then_0
              (Utilities|FlowControl|DoOnce false
                (:Completed
                  (Audio|PlaySoundatLocation "/Game/Blueprints/Audio/SFX_Final/Key/Key_Unlock.Key_Unlock" _returnvalue "0, 0, 0" 1.0 1.0 0.0 0 0 0 0))))
            (:then_1
              (|CallParentFunction Hit :!label _label_2)
              (CallFunction|VerifyBehind/InFront)
              (bind _output_get (Variables|Default|SetPlayer_T (Transformation|GetActorTransform (Variables|Default|GetPlayer_Ref))))
              (Components|Timeline|SetNewTime (Variables|Default|GetTimeline) 0.0)
              (bind _alpha_move (Timeline|Timeline Play)
                (:Update
                  (Transformation|SetActorTransform (Variables|Default|GetPlayer_Ref) (Math|Transform|Lerp(Transform) (Variables|Default|GetPlayer_T) (Math|Transform|MakeTransform (Math|Vector|MakeVector (.x (.location _d_player_t)) (.y (.location _d_player_t)) (.z (.location _output_get))) (.rotation _d_player_t) (.scale _output_get)) _alpha_move)))))))
        (else
          (goto _label)))
      (else
        (Audio|PlaySoundatLocation "/Game/Blueprints/Audio/SFX_Final/Key/Key_Locked.Key_Locked" _returnvalue "0, 0, 0" 1.0 1.0 0.0 0 0 0 0)
        (if (Variables|Default|GetDo_Anim_Lock)
          (CallFunction|AnimLocked))))
    (else
      (Variables|Default|SetHas%20Key%20? true)
      (goto _label_2))))

(event EventDrop
  (|CallParentFunction)
  (Audio|Components|Audio|Stop (Variables|Default|GetTimeline)))

(fn ConstructionScript
  (bind _bp_wheel (Variables|Default|GetBP_Wheel))
  (bind _childactor (Variables|/Script/Engine.ChildActorComponent|GetChildActor _bp_wheel))
  (bind _asbp_wheel (Utilities|Casting|CastToBP_Wheel _childactor))
  (|CallParentFunction)
  (Variables|/Game/Blueprints/BP_Object/BP_Wheel.BP_Wheel_C|SetLinkedActor _asbp_wheel self)
  (Collision|SetCollisionEnabled (Variables|/Game/Blueprints/BP_Object/BP_BaseObject.BP_BaseObject_C|GetMainMesh _asbp_wheel) "NoCollision"))