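; BP_PushingGrid is an interactable grid object that the player pushes over from inside or moves aside from outside.
; RemoveGrid picks the side via PushFromInterior and marks the grid opened, or only prints a debug string if Stop is set.
; Timelines scaled by duration disable Pawn blocking, then incrementally tilt the grid or slide it along Arrow until player Pourcentage exceeds 0.99.
; Separate events aim the player's view at LockViewPoint and restore it.
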(event Custom|RemoveGrid
  (if (Variables|Default|GetStop)
    (Development|PrintString "HelloHelloHelloHello")
    (elif (Variables|Default|GetPushFromInterior?)
      (CallFunction|PushingfromInside)
      (Variables|Default|SetHasBeenOpen? true)
      (else
        (CallFunction|PushingfromOutside)
        (Variables|Default|SetHasBeenOpen? true)))))

(event Custom|PushingFromOutside
  (bind _grid (Variables|Default|GetGrid))
  (bind _grid_2 (Variables|Default|GetGrid))
  (bind _returnvalue (Transformation|GetWorldLocation _grid_2))
  (bind _returnvalue_2 (Transformation|GetWorldRotation _grid))
  ;[1 1 1] Pushing From Outside
  (Components|Timeline|SetPlayRate (Variables|Default|GetMoveAsideGrid) (/ 1.0 (Variables|Default|GetMoveTime)))
  (Collision|SetCollisionResponsetoChannel (Variables|Default|GetGrid) "ECC_Pawn" "ECR_Ignore")
  (bind _rotation (Timeline|MoveAsideGrid Play)
    (:Update
      (if (not (> (Variables|/Game/Blueprints/BP_Player.BP_Player_C|GetPourcentage (.AsBP%20Player (Utilities|Casting|CastToBP_Player (Game|GetPlayerCharacter 0)))) 0.99))
        (Transformation|SetWorldLocationAndRotation (Variables|Default|GetGrid) (Math|Vector|Lerp(Vector) _returnvalue (+ _returnvalue (* (Math|Vector|GetForwardVector (Variables|Default|GetArrow)) (Variables|Default|GetSideLength))) _rotation) (Math|Rotator|Lerp(Rotator) (Transformation|GetWorldRotation (Variables|Default|GetGrid)) (Math|Rotator|MakeRotator (.roll _returnvalue_2) (- (.pitch _returnvalue_2) 0.25) (.yaw _returnvalue_2)) _rotation) false false)))))

(event Custom|Stop%20Lock%20View%20Look
  ;[0.2579 0.05517 0.2604] Stop Lock View Lock
  (bind _asbp_player (Utilities|Casting|CastToBP_Player (Game|GetPlayerCharacter 0)))
  (Pawn|SetControlRotation (Game|GetPlayerController 0) (Class|SpringArmComponent|GetTargetRotation (Variables|/Game/Blueprints/BP_Player.BP_Player_C|GetSpringArm _asbp_player))))

(event Custom|PushingFromInside
  (bind _grid (Variables|Default|GetGrid))
  (bind _grid_2 (Variables|Default|GetGrid))
  (bind _returnvalue (Transformation|GetWorldRotation _grid_2))
  (bind _returnvalue_2 (Transformation|GetWorldLocation _grid))
  ;[1 0.5094 0.4195] Pushing From Inside
  (Components|Timeline|SetPlayRate (Variables|Default|GetGridPush) (/ 1.0 (Variables|Default|GetPushTime)))
  (Collision|SetCollisionResponsetoChannel (Variables|Default|GetGrid) "ECC_Pawn" "ECR_Ignore")
  (bind _rotation (Timeline|GridPush Play)
    (:Update
      (Transformation|SetWorldLocationAndRotation (Variables|Default|GetGrid) (Math|Vector|Lerp(Vector) (Transformation|GetWorldLocation (Variables|Default|GetGrid)) (Math|Vector|MakeVector (.x _returnvalue_2) (.y _returnvalue_2) (.z _returnvalue_2)) _rotation) (Math|Rotator|Lerp(Rotator) (Transformation|GetWorldRotation (Variables|Default|GetGrid)) (Math|Rotator|MakeRotator (+ (.roll _returnvalue) 5.5) (.pitch _returnvalue) (.yaw _returnvalue)) _rotation) false false))))

(event Custom|Lock%20Look
  ;[1 1 1] Lock Look
  (bind _asbp_player (Utilities|Casting|CastToBP_Player (Game|GetPlayerCharacter 0)))
  (Pawn|SetControlRotation (Game|GetPlayerController 0) (Math|Rotator|FindLookatRotation (Transformation|GetWorldLocation (Variables|/Game/Blueprints/BP_Player.BP_Player_C|GetSpringArm _asbp_player)) (Transformation|GetWorldLocation (Variables|Default|GetLockViewPoint)))))

(event EventBeginPlay
  (Variables|Default|SetHasBeenOpen? false))

(fn ConstructionScript
  (Variables|Default|SetTypeObject "NewEnumerator0"))