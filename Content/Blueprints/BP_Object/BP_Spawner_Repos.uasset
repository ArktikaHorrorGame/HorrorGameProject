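; BP_Spawner_Repos is an activatable vent spawner that releases a referenced monster to patrol for a limited time, then sends it back.
; On activation it nulls the monster's state, moves its capsule to a scene point and plays a vent-exit montage.
; When the montage completes, the monster patrols a given route until a timer switches it to guard mode, targeting the vent entrance as its return post.
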(event Custom|ActivateMonster
  (bind _monstre_ref (Variables|Default|GetMonstre_Ref))
  ;[1 1 1] il faudra l'activer a la fin de l'anim avec un notify
  (Actor|Tick|SetActorTickEnabled true)
  (Variables|/Game/Blueprints/EnemyAI/BP_MonstreAI.BP_MonstreAI_C|SetPatrol_Speed _monstre_ref (Variables|Default|GetPatrol_Speed))
  (Default|ChangetoPatrol _monstre_ref (Variables|Default|GetIndex%20Patrol))
  (Variables|/Game/Blueprints/EnemyAI/BP_MonstreAI.BP_MonstreAI_C|SetCurrent_Patrol_Point _monstre_ref -1)
  (Utilities|Time|SetTimerbyEvent (delegate Custom|GoBackVent) (Variables|Default|GetTime_ReturnVent)))

(event Custom|GoBackVent
  (bind _monstre_ref (Variables|Default|GetMonstre_Ref))
  (bind _entre_vent (Variables|Default|GetEntre_Vent))
  (bind _returnvalue (Transformation|GetWorldLocation _entre_vent))
  (Variables|/Game/Blueprints/EnemyAI/BP_MonstreAI.BP_MonstreAI_C|SetGuardPostPosition _monstre_ref (Math|Vector|MakeVector (.x _returnvalue) (.y _returnvalue) (.z _returnvalue)))
  (Default|ResetBacktoVent (Variables|Default|GetMonstre_Ref) (Transformation|GetWorldRotation (Variables|Default|GetEntre_Vent)))
  (Default|ChangetoGuard _monstre_ref)
  (Variables|/Game/Blueprints/EnemyAI/BP_MonstreAI.BP_MonstreAI_C|SetReturnVent? _monstre_ref true)
  (Actor|Tick|SetActorTickEnabled false))

(event EventBeginPlay)

(event Collision|EventActorBeginOverlap
  (params (OtherActor :type Actor%20Object%20Reference)))

(event EventObjectActivate
  (bind _monstre_ref (Variables|Default|GetMonstre_Ref))
  (Default|ChangetoNull _monstre_ref)
  (Transformation|SetWorldLocation (Variables|/Script/Engine.Character|GetCapsuleComponent _monstre_ref) (Transformation|GetWorldLocation (Variables|Default|GetScene)) false false)
  ;[1 1 1] Anim sortie vent
  (Animation|Montage|PlayMontage (Variables|/Script/Engine.Character|GetMesh _monstre_ref) "/Game/Blueprints/Animation/Sortie_Vent_Lent/Sortie_vent_lente_Pose_Bake_Anim_Montage.Sortie_vent_lente_Pose_Bake_Anim_Montage"
    (:OnCompleted
      (CallFunction|ActivateMonster))))

(fn ConstructionScript)