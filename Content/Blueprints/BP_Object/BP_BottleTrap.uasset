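; Bottle trap actor that is launched when its trigger box is overlapped and shatters when it hits a trap detection area.
; Any overlap on the Box applies a large diagonal force to the StaticMesh at the world location cached in RefPoint on BeginPlay.
; When the mesh overlaps a BP_TrapDetectionArea, the actor destroys itself and spawns ShatterBottle at its actor location and rotation.
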(event OnComponentBeginOverlap(StaticMesh)
  (params (OverlappedComponent :type Primitive%20Component%20Object%20Reference) (OtherActor :type Actor%20Object%20Reference) (OtherComp :type Primitive%20Component%20Object%20Reference) (OtherBodyIndex :type Integer) (bFromSweep :type Boolean) (SweepResult :type Hit%20Result%20Structure%20%28by%20ref%29))
  (Utilities|Casting|CastToBP_TrapDetectionArea OtherActor)
  (Actor|DestroyActor)
  (Game|SpawnActorfromClass "/Game/FirstPerson/AllMeca/Chaos/ShatterBottle.ShatterBottle_C" (Math|Transform|MakeTransform (Transformation|GetActorLocation) (Transformation|GetActorRotation) "1.000000,1.000000,1.000000") "Undefined" "MultiplyWithRoot" 0 0))

(event OnComponentBeginOverlap(Box)
  (params (OverlappedComponent :type Primitive%20Component%20Object%20Reference) (OtherActor :type Actor%20Object%20Reference) (OtherComp :type Primitive%20Component%20Object%20Reference) (OtherBodyIndex :type Integer) (bFromSweep :type Boolean) (SweepResult :type Hit%20Result%20Structure%20%28by%20ref%29))
  (Class|PrimitiveComponent|AddForceatLocation (Variables|Default|GetStaticMesh) (Math|Vector|MakeVector 7.5e+05 7.5e+05 7.5e+05) (.location (Variables|Default|GetRefPoint)) "None"))

(event EventBeginPlay
  ;[0.3542 0 0.2611] Set Ref Point Position
  (Variables|Default|SetRefPoint (Math|Transform|MakeTransform (Transformation|GetWorldLocation (Variables|Default|GetStaticMesh)) "0, 0, 0" "1.000000,1.000000,1.000000")))

(fn ConstructionScript)