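; BP_Telegraph0 is a grabbable telegraph that locks the player and camera onto itself for mouse-cursor use.
; Grabbed shows the cursor, disables player input and runs a timeline easing the character to an actor-relative offset with a fixed world rotation.
; While grabbed, Tick aims control rotation from the BP_Player spring arm at the telegraph and sets Grabbing.
; Tick also debug-prints mouse X; no release is wired, as EnableInput is unreachable.
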(event Custom|Pos_For_Telegraph
  (bind _pos (Variables|Default|GetPos))
  (bind _newtrack_0 (Timeline|Timeline PlayFromStart)
    (:Update
      (Transformation|SetActorLocationAndRotation (Game|GetPlayerCharacter 0) (Math|Vector|Lerp(Vector) (Transformation|GetWorldLocation (Variables|/Script/Engine.Actor|GetRootComponent (Game|GetPlayerCharacter 0))) (Math|Transform|TransformLocation (Transformation|GetActorTransform) (.location _pos)) _newtrack_0) (.rotation _pos)))))

(event Custom|Verify%20Lock%20look
  ;[1 1 1] Verify Lock Cam
  (if (not (not (Variables|Default|GetGrabbeddd)))
    (CallFunction|LockLook)))

(event Custom|Lock%20look
  ;[1 1 1] Lock Cam
  (bind _asbp_player (Utilities|Casting|CastToBP_Player (Game|GetPlayerCharacter 0)))
  (Pawn|SetControlRotation (Game|GetPlayerController 0) (Math|Rotator|FindLookatRotation (Transformation|GetWorldLocation (Variables|/Game/Blueprints/BP_Player.BP_Player_C|GetSpringArm _asbp_player)) (Transformation|GetWorldLocation (Variables|Default|GetTelegraph))))
  (Variables|/Game/Blueprints/BP_Player.BP_Player_C|SetGrabbing%20? _asbp_player true))

(event Collision|EventActorBeginOverlap
  (params (OtherActor :type Actor%20Object%20Reference)))

(event EventBeginPlay
  (Variables|Default|SetPos (Math|Transform|MakeTransform "76.000000,-35.000000,135.000000" "0.000000,90.000000,8.000000" "1.000000,1.000000,1.000000")))

(event EventTick
  (params (DeltaSeconds :type Float%20%28single-precision%29))
  ;[1 1 1] Update
  (Utilities|FlowControl|Sequence
    (:then_0
      (Development|PrintString (Utilities|String|ToString(Float) (.LocationX (Class|WidgetLayoutLibrary|GetMousePositionScaledbyDPI (Game|GetPlayerController 0)))) true true "(R=0.000000,G=0.216624,B=1.000000,A=1.000000)" 0.0))
    (:then_1
      (CallFunction|VerifyLockLook))))

(event EventGrabed
  (params (GrabPoint_Location :type Scene%20Component%20Object%20Reference) (Cam%20/Camera%20Arm :type Spring%20Arm%20Component%20Object%20Reference) (BP_Player_Ref :type BP%20Player%20Object%20Reference))
  ;[1 0.6387 0.2958] Lock cam and active mouse
  (Variables|Default|SetGrabbeddd true)
  (CallFunction|PosforTelegraph)
  (Variables|/Script/Engine.PlayerController|SetbShowMouseCursor (Game|GetPlayerController 0) true)
  (Input|DisableInput (Game|GetPlayerCharacter 0) 0))

(fn ConstructionScript
  (|CallParentFunction))