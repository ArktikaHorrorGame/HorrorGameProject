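; BP_Cachette is a hiding spot ("cachette") that moves the player inside when they interact with it.
; Interaction disables player movement, swings the optional door open, then runs Hide and closes the door afterward.
; Hide uses a timeline to lerp the player to HideTransform, halving Z scale for short objects, while interpolating camera yaw toward LookTransform.
; Player overlap with Box_Collision also calls Hide directly; the file has no exit logic.
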(event OnComponentBeginOverlap(Box_Collision)
  (params (OverlappedComponent :type Primitive%20Component%20Object%20Reference) (OtherActor :type Actor%20Object%20Reference) (OtherComp :type Primitive%20Component%20Object%20Reference) (OtherBodyIndex :type Integer) (bFromSweep :type Boolean) (SweepResult :type Hit%20Result%20Structure%20%28by%20ref%29))
  (Utilities|Casting|CastToBP_Player OtherActor)
  (CallFunction|Hide))

(event OnComponentEndOverlap(Box_Collision)
  (params (OverlappedComponent :type Primitive%20Component%20Object%20Reference) (OtherActor :type Actor%20Object%20Reference) (OtherComp :type Primitive%20Component%20Object%20Reference) (OtherBodyIndex :type Integer)))

(event Custom|OpenDoor
  (bind _smooth_open (Timeline|Timeline_0 Play)
    (:Update
      (Transformation|SetRelativeRotation (Variables|Default|GetSM_Porte_Cachette) (Math|Rotator|MakeRotator 0.0 0.0 (Math|Float|Lerp (Variables|Default|GetStart%20Angle) (Variables|Default|GetEnd%20Angle) _smooth_open)) false false))
    (:Finished
      (Variables|Default|SetDoorIsOpen true)
      (CallFunction|Hide))))

(event Custom|Hide
  (bind _ref_player (Variables|Default|GetRef_Player))
  (bind _returnvalue (Pawn|GetController _ref_player))
  (bind _returnvalue_2 (Pawn|GetControlRotation _returnvalue :!class /Script/Engine.Controller))
  (bind (_roll _pitch) (Math|Rotator|BreakRotator _returnvalue_2))
  (bind _smooth_transition (Timeline|Timeline Play)
    (:Update
      (Transformation|SetActorTransform _ref_player (Math|Transform|Lerp(Transform) (Variables|Default|GetActorCurrentTransform) (Variables|Default|GetActorHideTransform) _smooth_transition))
      (Pawn|SetControlRotation _returnvalue (Math|Rotator|MakeRotator _roll _pitch (.yaw (Math|Interpolation|RInterpTo _returnvalue_2 (Math|Rotator|FindLookatRotation (Transformation|GetWorldLocation (Variables|/Game/Blueprints/BP_Player.BP_Player_C|GetCamera _ref_player)) (Transformation|GetWorldLocation (Variables|Default|GetLook_Transform))) (Utilities|Time|GetWorldDeltaSeconds) 0.0)))))
    (:Finished
      (if (Variables|Default|GetDoorIsOpen)
        (CallFunction|CloseDoor)))))

(event Custom|CloseDoor
  (bind _smooth_open (Timeline|Timeline_0 Reverse)
    (:Update
      (Transformation|SetRelativeRotation (Variables|Default|GetSM_Porte_Cachette) (Math|Rotator|MakeRotator 0.0 0.0 (Math|Float|Lerp (Variables|Default|GetStart%20Angle) (Variables|Default|GetEnd%20Angle) _smooth_open)) false false))
    (:Finished
      (Variables|Default|SetDoorIsOpen true)
      (CallFunction|Hide))))

(event EventInteraction
  (bind _asbp_player (Utilities|Casting|CastToBP_Player (Game|GetPlayerCharacter 0)))
  (bind _output_get (Variables|Default|SetRef_Player _asbp_player))
  (Pawn|Components|CharacterMovement|DisableMovement (Variables|/Script/Engine.Character|GetCharacterMovement _output_get))
  (Variables|Default|SetActorCurrentTransform (Transformation|GetActorTransform _asbp_player))
  (if (not (Variables|Default|GetHasDoor%20?))
    (CallFunction|Hide)
    (else
      (CallFunction|OpenDoor))))

(event EventBeginPlay
  (if (Variables|Default|GetShortObject)
    (Variables|Default|SetPlayerScale 0.5)
    (else
      (Variables|Default|SetPlayerScale 1.0)))
  (Variables|Default|SetActorHideTransform (Math|Transform|MakeTransform (Transformation|GetWorldLocation (Variables|Default|GetHide_Transform)) "0, 0, 0" (Math|Vector|MakeVector 1.0 1.0 (Variables|Default|GetPlayerScale)))))

(fn ConstructionScript)