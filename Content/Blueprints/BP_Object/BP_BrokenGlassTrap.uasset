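; Broken glass trap that alerts the monster when the player overlaps its box.
; If the monster is not already chasing, it sets the chase flag, plays a breaking-glass sound and sends an activate message to the linked vent.
; A sphere trace at the player gives the location for an extra sound and AI noise event, fired only if a capsule velocity component exceeds a positive threshold.
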(event OnComponentBeginOverlap(Box)
  (params (OverlappedComponent :type Primitive%20Component%20Object%20Reference) (OtherActor :type Actor%20Object%20Reference) (OtherComp :type Primitive%20Component%20Object%20Reference) (OtherBodyIndex :type Integer) (bFromSweep :type Boolean) (SweepResult :type Hit%20Result%20Structure%20%28by%20ref%29))
  (bind _returnvalue (Game|GetPlayerCharacter 0))
  (bind _monstre_ref (Variables|Default|GetMonstre_Ref))
  (bind _rootcomponent (Variables|/Script/Engine.Actor|GetRootComponent _returnvalue))
  (bind _returnvalue_2 (Transformation|GetWorldLocation _rootcomponent))
  (Utilities|Casting|CastToBP_Player OtherActor)
  (if (not (Variables|/Game/Blueprints/EnemyAI/BP_MonstreAI.BP_MonstreAI_C|GetIsChasing? _monstre_ref))
    (Variables|/Game/Blueprints/EnemyAI/BP_MonstreAI.BP_MonstreAI_C|SetIsChasing? _monstre_ref true)
    (Audio|PlaySoundatLocation "/Game/FirstPerson/AllMeca/GlassPane/Glass_Breaking_Sound_Effect.Glass_Breaking_Sound_Effect" (Transformation|GetActorLocation) (Transformation|GetActorRotation) 0.2 1.0 0.0 0 0 0 0)
    (Class|BPIObjectActivate|ObjectActivate(Message) (Variables|Default|GetVent))
    (bind _outhit (Collision|SphereTraceByChannel _returnvalue_2 _returnvalue_2 3e+01 "TraceTypeQuery1" true 0 "ForDuration"))
    (bind _returnvalue_3 (Physics|GetPhysicsLinearVelocity (Variables|/Script/Engine.Character|GetCapsuleComponent (Game|GetPlayerCharacter 0)) "None"))
    (if (Math|Boolean|ORBoolean (> (.x _returnvalue_3) 65.0) (> (.y _returnvalue_3) 65.0) (> (.z _returnvalue_3) 65.0))
      (Audio|SpawnSoundatLocation (Variables|Default|GetSound) (.location _outhit) "0, 0, 0" 1.0 1.0 0.0 0 0)
      (Class|AISenseHearing|ReportNoiseEvent (.location _outhit) 1.0 self 3e+03 (Utilities|Name|EnumtoName (Variables|Default|GetSound_Type))))))

(fn ConstructionScript)