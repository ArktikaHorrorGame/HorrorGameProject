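; Conduit trigger actor that pulls the player to a set spot and toggles the player's crawling system.
; On first overlap, a Timeline lerps the player from its current location toward the FinalPos offset and applies that rotation.
; Leaving the box calls CrawlingSystem again and clears the InsideConduit guard.
; Input is disabled when the move starts but re-enabled on every Timeline update rather than on finish.
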(event OnComponentEndOverlap(Box)
  (params (OverlappedComponent :type Primitive%20Component%20Object%20Reference) (OtherActor :type Actor%20Object%20Reference) (OtherComp :type Primitive%20Component%20Object%20Reference) (OtherBodyIndex :type Integer))
  (bind _asbp_player (Utilities|Casting|CastToBP_Player OtherActor))
  (Default|CrawlingSystem _asbp_player)
  (Variables|Default|SetInsideConduit false))

(event OnComponentBeginOverlap(Box)
  (params (OverlappedComponent :type Primitive%20Component%20Object%20Reference) (OtherActor :type Actor%20Object%20Reference) (OtherComp :type Primitive%20Component%20Object%20Reference) (OtherBodyIndex :type Integer) (bFromSweep :type Boolean) (SweepResult :type Hit%20Result%20Structure%20%28by%20ref%29))
  (Utilities|Casting|CastToBP_Player OtherActor)
  (if (not (Variables|Default|GetInsideConduit))
    (CallFunction|Hiding)
    (Default|CrawlingSystem (stale EventBeginPlay _asbp_player))
    (Variables|Default|SetInsideConduit true)))

(event Custom|Hiding
  (bind _final_pos (Variables|Default|GetFinal_Pos))
  (Input|DisableInput 0)
  (Variables|Default|SetInput? false)
  (bind _newtrack_0 (Timeline|Timeline PlayFromStart)
    (:Update
      (Transformation|SetActorLocationAndRotation (stale EventBeginPlay _asbp_player) (Math|Vector|Lerp(Vector) (Transformation|GetWorldLocation (Variables|/Script/Engine.Actor|GetRootComponent (stale EventBeginPlay _asbp_player))) (Math|Transform|TransformLocation (Transformation|GetActorTransform) (.location _final_pos)) _newtrack_0) (.rotation _final_pos))
      (Input|EnableInput 0))))

(event EventBeginPlay
  (bind _asbp_player (Utilities|Casting|CastToBP_Player (Game|GetPlayerCharacter 0)))
  (Variables|Default|SetInsideConduit false))

(fn ConstructionScript)