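; Valve-operated door or mechanism whose hinge constraint stays locked until its matching key object is fitted, when a key is required.
; BeginPlay locks the physics constraint's swing and sets the main mesh rotation.
; A hit from the assigned BP_Valve_Key makes the player release it, destroys it and reveals the wooden wheel.
; Tick polls the key flag and, once set, switches the hinge to limited swing a single time.
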(event OnComponentHit(MainMesh)
  (params (HitComponent :type Primitive%20Component%20Object%20Reference) (OtherActor :type Actor%20Object%20Reference) (OtherComp :type Primitive%20Component%20Object%20Reference) (NormalImpulse :type Vector :default "0, 0, 0") (Hit :type Hit%20Result%20Structure%20%28by%20ref%29))
  (bind _asbp_valve_key (Utilities|Casting|CastToBP_Valve_Key OtherActor))
  (if (== _asbp_valve_key (Variables|Default|GetValveKey))
    (Variables|Default|SetHas%20Key%20? true)
    (bind _asbp_player (Utilities|Casting|CastToBP_Player (Game|GetPlayerCharacter 0)))
    (Default|Release _asbp_player)
    (Actor|DestroyActor (Variables|Default|GetValveKey))
    (Development|SetHiddeninGame (Variables|Default|Getwooden_wheel) false false)))

(event Custom|Verify%20Valve
  (if (Variables|Default|GetHas%20Key%20?)
    (Utilities|FlowControl|DoOnce false
      (:Completed
        (Class|PhysicsConstraintComponent|SetAngularSwing1Limit (Variables|Default|GetHinges) "ACM_Limited" 45.0)))))

(event EventBeginPlay
  (if (Variables|Default|GetNeed%20Key%20?)
    (Class|PhysicsConstraintComponent|SetAngularSwing1Limit (Variables|Default|GetHinges) "ACM_Locked" 0.0)
    (Transformation|SetRelativeRotation (Variables|Default|GetMainMesh) "0.000000,45.000000,0.000000" false false))
  (|CallParentFunction))

(event Collision|EventActorBeginOverlap
  (params (OtherActor :type Actor%20Object%20Reference)))

(event EventTick
  (params (DeltaSeconds :type Float%20%28single-precision%29))
  (CallFunction|VerifyValve)
  (|CallParentFunction DeltaSeconds))

(fn ConstructionScript
  (|CallParentFunction))