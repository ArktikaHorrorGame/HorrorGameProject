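; BP_Prone is a grabbable conduit entry that moves the player inside and triggers the player's crawling system.
; On the first grab, it starts a timeline positioning the player relative to a local start point, calls CrawlingSystem and schedules Hiding one second later.
; Hiding uses the SmoothTP timeline to lerp the player to the local end point, toggling input around the move.
; InsideConduit blocks further grabs and is never cleared here.
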(event Custom|Hiding
  (bind _final_pos (Variables|Default|GetFinal_Pos))
  (Input|DisableInput 0)
  (Variables|Default|SetInput? false)
  (bind _newtrack_0 (Timeline|SmoothTP PlayFromStart)
    (:Update
      (Transformation|SetActorLocationAndRotation (Variables|Default|GetRef_Player) (Math|Vector|Lerp(Vector) (Transformation|GetWorldLocation (Variables|/Script/Engine.Actor|GetRootComponent (Variables|Default|GetRef_Player))) (Math|Transform|TransformLocation (Transformation|GetActorTransform) (.location _final_pos)) _newtrack_0) (.rotation _final_pos))
      (Input|EnableInput 0)
      (Variables|Default|SetInput? true))))

(event Custom|Start_Pos
  (bind _starting_pos (Variables|Default|GetStarting_Pos))
  (bind _newtrack_0 (Timeline|Timeline PlayFromStart)
    (:Update
      (Transformation|SetActorLocationAndRotation (Variables|Default|GetRef_Player) (Math|Vector|Lerp(Vector) (Math|Transform|TransformLocation (Transformation|GetActorTransform) (.location _starting_pos)) (Transformation|GetWorldLocation (Variables|/Script/Engine.Actor|GetRootComponent (Variables|Default|GetRef_Player))) _newtrack_0) (.rotation _starting_pos)))))

(event EventGrabed
  (params (GrabPoint_Location :type Scene%20Component%20Object%20Reference) (Cam%20/Camera%20Arm :type Spring%20Arm%20Component%20Object%20Reference) (BP_Player_Ref :type BP%20Player%20Object%20Reference))
  ;[0.5 0.281 0.111] When clicked
  (if (not (Variables|Default|GetInsideConduit))
    (CallFunction|StartPos)
    (Utilities|Time|SetTimerbyEvent (delegate Custom|Hiding) 1.0)
    (Default|CrawlingSystem BP_Player_Ref)
    (Variables|Default|SetInsideConduit true)))

(event EventBeginPlay
  (bind _asbp_player (Utilities|Casting|CastToBP_Player (Game|GetPlayerCharacter 0)))
  (Variables|Default|SetRef_Player _asbp_player)
  (Variables|Default|SetInsideConduit false)
  (Variables|Default|SetFinal_Pos (Math|Transform|MakeTransform "0.000000,-81.500000,-13.300000" "0, 0, 0" "1.000000,1.000000,1.000000"))
  (Variables|Default|SetStarting_Pos (Math|Transform|MakeTransform "0.000000,57.500000,-10.000000" "0.000000,0.000000,0.000000" "1.000000,1.000000,1.000000")))

(fn ConstructionScript
  (|CallParentFunction))