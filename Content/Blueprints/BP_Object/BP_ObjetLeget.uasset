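; BP_ObjetLeget is a child Blueprint for an object meant to be grabbed and released by the player.
; Its Grabed, Released and Tick events are empty, and the construction script only calls the parent's.
; Disconnected leftover nodes would toggle a TestGrab flag and drive the player's PhysicsHandle toward a smoothed point in front of the spring arm at Zoom distance, matching control rotation, but they never run.
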(event EventBeginPlay)

(event Collision|EventActorBeginOverlap
  (params (OtherActor :type Actor%20Object%20Reference)))

(event EventTick
  (params (DeltaSeconds :type Float%20%28single-precision%29)))

(event EventGrabed
  (params (GrabPoint_Location :type Scene%20Component%20Object%20Reference) (Cam%20/Camera%20Arm :type Spring%20Arm%20Component%20Object%20Reference) (BP_Player_Ref :type BP%20Player%20Object%20Reference)))

(event EventReleased)

(fn ConstructionScript
  (|CallParentFunction))