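; Heavy physics object that the player grabs and drags around with mouse and movement, walking slower while holding it.
; Each tick while grabbed, it locks the camera onto TouchSpot and turns camera-relative mouse delta plus pawn velocity into a clamped, mass-scaled force on the mesh.
; Exceeding MaxDistance calls the player's far release; Released restores control rotation and speed.
; Hits from a held BP_GrabObjet switch off its physics simulation.
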(event OnComponentHit(StaticMeshComponent)
  (params (HitComponent :type Primitive%20Component%20Object%20Reference) (OtherActor :type Actor%20Object%20Reference) (OtherComp :type Primitive%20Component%20Object%20Reference) (NormalImpulse :type Vector :default "0, 0, 0") (Hit :type Hit%20Result%20Structure%20%28by%20ref%29))
  (bind _staticmeshcomponent (Variables|Default|GetStaticMeshComponent))
  (bind _asbp_grab_objet (Utilities|Casting|CastToBP_GrabObjet OtherActor))
  (if (Variables|/Game/Blueprints/BP_Object/BP_GrabObjet.BP_GrabObjet_C|GetGrabbed? _asbp_grab_objet)
    (Physics|SetSimulatePhysics _staticmeshcomponent false)
    (else
      (Physics|SetSimulatePhysics _staticmeshcomponent true))))

(event Custom|Stop%20Lock%20Look
  ;[1 1 1] Stop Lock Cam
  (bind _asbp_player (Utilities|Casting|CastToBP_Player (Game|GetPlayerCharacter 0)))
  (Pawn|SetControlRotation (Game|GetPlayerController 0) (Class|SpringArmComponent|GetTargetRotation (Variables|/Game/Blueprints/BP_Player.BP_Player_C|GetSpringArm _asbp_player))))

(event Custom|Verify%20Lock%20look
  ;[1 1 1] Verify lock Cam
  (if (not (not (Variables|Default|GetGrabbed)))
    (CallFunction|LockLook)))

(event Custom|Lock%20look
  ;[1 1 1] Lock Cam
  (bind _asbp_player (Utilities|Casting|CastToBP_Player (Game|GetPlayerCharacter 0)))
  (Pawn|SetControlRotation (Game|GetPlayerController 0) (Math|Rotator|FindLookatRotation (Transformation|GetWorldLocation (Variables|/Game/Blueprints/BP_Player.BP_Player_C|GetSpringArm _asbp_player)) (Transformation|GetWorldLocation (Variables|Default|GetTouchSpot))))
  (Variables|/Game/Blueprints/BP_Player.BP_Player_C|SetGrabbing%20? _asbp_player true))

(event Custom|Force%20impulse%20Move
  (bind _returnvalue (Game|GetPlayerController 0))
  (bind _staticmeshcomponent (Variables|Default|GetStaticMeshComponent))
  (bind (_deltax _deltay) (Class|PlayerController|GetInputMouseDelta _returnvalue))
  (bind _playercameramanager (Variables|/Script/Engine.PlayerController|GetPlayerCameraManager _returnvalue))
  ;[1 1 1] Recup Mouse Input To Make the Movement
  (if (Variables|Default|GetGrabbed)
    (Variables|Default|SetMouseDeltaX _deltax)
    (Variables|Default|SetMouseDeltaY _deltay)
    (Variables|Default|SetForce (+ (* (* (* (Transformation|GetActorRightVector _playercameramanager) (Variables|Default|GetMouseDeltaX)) 1e+02) (Class|PlayerController|GetDeprecatedInputYawScale _returnvalue)) (* (* (* (Transformation|GetActorForwardVector _playercameramanager) (Variables|Default|GetMouseDeltaY)) 1e+02) (* (Class|PlayerController|GetDeprecatedInputPitchScale _returnvalue) -1.0))))
    ;[1 1 1] Use The player Movement To make Movement (Velocity)
    (bind _output_get (Variables|Default|SetForce (+ (Variables|Default|GetForce) (* (Transformation|GetVelocity (Variables|Default|GetPlayer%20Pawn%20Ref)) 2.0))))
    (Variables|Default|SetForce (Math|Vector|MakeVector (.x _output_get) (.y _output_get) (.z (Variables|/Script/Engine.SceneComponent|GetRelativeLocation (Variables|Default|GetObject_Handel)))))
    (Transformation|AttachComponentToComponent (Variables|Default|GetTouchSpot) (Variables|Default|GetStaticMeshComponent) "None" "KeepWorld" "KeepWorld" "KeepWorld" true)
    ;[1 1 1] Lock The Max Force
    (if (> (Math|Vector|Distance(Vector) (Math|Vector|VectorZero) (Variables|Default|GetForce)) (Variables|Default|GetMaxForce))
      (Variables|Default|SetForce (* (Math|Vector|Normalize (Variables|Default|GetForce)) (Variables|Default|GetMaxForce))))
    ;[1 1 1] Apply the Force at the Center of the mass so will always work whanever you interact with the door
    (Physics|AddForce _staticmeshcomponent (* (* (Variables|Default|GetForce) (Variables|Default|GetForceobject)) (Physics|GetMass _staticmeshcomponent)) "None" false)))

(event Custom|Distance_Verification
  (bind _playerbp_ref (Variables|Default|GetPlayerBP_Ref))
  ;[1 1 1] Verification Distance
  (if (Variables|Default|GetGrabbed)
    (if (> (Math|Vector|Distance(Vector) (Transformation|GetWorldLocation (Variables|Default|GetStaticMeshComponent)) (Transformation|GetWorldLocation (Variables|/Script/Engine.Character|GetMesh _playerbp_ref))) (Variables|Default|GetMax_Distance))
      (Default|ToFarRelease _playerbp_ref))))

(event EventTick
  (params (DeltaSeconds :type Float%20%28single-precision%29))
  ;[1 1 1] Event tick
  (CallFunction|VerifyLockLook)
  (CallFunction|ForceImpulseMove)
  (CallFunction|DistanceVerification))

(event EventReleased
  ;[1 1 1] Released
  (Variables|Default|SetGrabbed false)
  (Variables|/Game/Blueprints/BP_Player.BP_Player_C|SetGrabbing%20? (Variables|Default|GetPlayerBP_Ref) false)
  (CallFunction|StopLockLook)
  (Variables|/Script/Engine.CharacterMovementComponent|SetMaxWalkSpeed (Variables|/Script/Engine.Character|GetCharacterMovement (Game|GetPlayerCharacter 0)) 275.0))

(event EventGrabed
  (params (GrabPoint_Location :type Scene%20Component%20Object%20Reference) (Cam%20/Camera%20Arm :type Spring%20Arm%20Component%20Object%20Reference) (BP_Player_Ref :type BP%20Player%20Object%20Reference))
  ;[1 1 1] Grabed
  (Physics|SetSimulatePhysics (Variables|Default|GetStaticMeshComponent) true)
  (Variables|Default|SetCam%20/%20Camera%20Arm Cam%20/Camera%20Arm)
  (Variables|Default|SetPlayerBP_Ref BP_Player_Ref)
  (Variables|Default|SetGrabbed true)
  (Variables|Default|SetPlayer%20Pawn%20Ref (Pawn|GetControlledPawn (Game|GetPlayerController 0)))
  ;;[1 1 1] Block/Slow Movement when Moving object
  ;;;[1 1 1] Set 0 to block
  (Variables|/Script/Engine.CharacterMovementComponent|SetMaxWalkSpeed (Variables|/Script/Engine.Character|GetCharacterMovement (Game|GetPlayerCharacter 0)) 5e+01))

(fn ConstructionScript
  (|CallParentFunction))