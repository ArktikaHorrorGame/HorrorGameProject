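; Grabbable physics object that the player carries in front of the camera and can highlight through an overlap component.
; While grabbed, Tick interpolates a hold point at Zoom distance and drives the player's PhysicsHandle, optionally easing rotation toward control rotation plus an offset.
; Grabbing passes the object's throw power to the player or destroys the actor if flagged; release restores default zoom.
; HighLight overlaps toggle a material scalar parameter.
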(event OnComponentBeginOverlap(HighLight)
  (params (OverlappedComponent :type Primitive%20Component%20Object%20Reference) (OtherActor :type Actor%20Object%20Reference) (OtherComp :type Primitive%20Component%20Object%20Reference) (OtherBodyIndex :type Integer) (bFromSweep :type Boolean) (SweepResult :type Hit%20Result%20Structure%20%28by%20ref%29))
  (Rendering|Material|SetScalarParameterValueonMaterials (Variables|Default|GetStaticMeshComponent) "Highlight" 1.0))

(event OnComponentEndOverlap(HighLight)
  (params (OverlappedComponent :type Primitive%20Component%20Object%20Reference) (OtherActor :type Actor%20Object%20Reference) (OtherComp :type Primitive%20Component%20Object%20Reference) (OtherBodyIndex :type Integer))
  (Rendering|Material|SetScalarParameterValueonMaterials (Variables|Default|GetStaticMeshComponent) "Highlight" 0.0))

(event EventGrabed
  (params (GrabPoint_Location :type Scene%20Component%20Object%20Reference) (Cam%20/Camera%20Arm :type Spring%20Arm%20Component%20Object%20Reference) (BP_Player_Ref :type BP%20Player%20Object%20Reference))
  (Variables|Default|SetTest_Grab true)
  (Variables|/Game/Blueprints/BP_Player.BP_Player_C|SetMax_Throw_Power BP_Player_Ref (Utilities|Struct|BreakS_GrabObject_Info (Variables|Default|GetS_Object_Info)))
  (if (Variables|Default|GetDestroy%20it%20?)
    (Actor|DestroyActor)))

(event EventTick
  (params (DeltaSeconds :type Float%20%28single-precision%29))
  (bind _bp_player_ref (Variables|Default|GetBP%20Player%20Ref))
  (bind _camera (Variables|/Game/Blueprints/BP_Player.BP_Player_C|GetCamera _bp_player_ref))
  (Variables|Default|GetBP%20Player%20Ref
    (:then
      (if (Variables|Default|GetTest_Grab)
        (Variables|Default|SetWorldLoc (Transformation|GetWorldLocation _camera))
        (Variables|Default|SetWorldRot (Pawn|GetControlRotation _bp_player_ref :!class /Script/Engine.Pawn))
        (bind _output_get (Variables|Default|SetGrabWorldLoc (Math|Interpolation|VInterpTo (Variables|Default|GetGrabWorldLoc) (+ (Math|Vector|MakeVector (.x (Variables|Default|GetWorldLoc)) (.y (Variables|Default|GetWorldLoc)) (- (.z (Variables|Default|GetWorldLoc)) 2e+01)) (* (Math|Vector|GetForwardVector _camera) (Variables|Default|GetZoom))) (Utilities|Time|GetWorldDeltaSeconds) (Variables|Default|GetLocationInterpSpeed))))
        (bind _rotation (CallFunction|AutoRotation))
        (Class|PhysicsHandleComponent|SetTargetLocationandRotation (Variables|/Game/Blueprints/BP_Player.BP_Player_C|GetPhysicsHandle (Variables|Default|GetBP%20Player%20Ref)) _output_get _rotation)))
    (:else)))

(event EventBeginPlay
  (|CallParentFunction)
  (Variables|Default|SetZoom_Base (Variables|Default|GetZoom)))

(event EventReleased
  (Variables|Default|SetTest_Grab false)
  (Variables|Default|SetZoom (Variables|Default|GetZoom_Base)))

(fn ConstructionScript
  (|CallParentFunction))

(fn AutoRotation
  (bind _s_autorotation (Variables|Default|GetS_AutoRotation))
  (bind _worldrot (Variables|Default|GetWorldRot))
  (bind (_roll _pitch _yaw) (Utilities|Struct|BreakS_AutoRotaion _s_autorotation))
  (bind (_roll_2 _pitch_2 _yaw_2) (Math|Rotator|BreakRotator _worldrot))
  (return (Math|Rotator|Lerp(Rotator) (Transformation|GetWorldRotation (Variables|Default|GetStaticMeshComponent)) (Math|Rotator|SelectRotator (Math|Rotator|MakeRotator (+ _roll_2 _roll) (+ _pitch_2 _pitch) (+ _yaw_2 _yaw)) (Transformation|GetWorldRotation (Variables|Default|GetStaticMeshComponent)) (Utilities|Struct|BreakS_AutoRotaion (Variables|Default|GetS_AutoRotation))) (Variables|Default|GetSmoothAutoRotation) true)))