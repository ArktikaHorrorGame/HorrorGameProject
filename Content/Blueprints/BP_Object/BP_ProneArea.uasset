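; Trigger box for a prone crawl area (conduit) that switches player and entrance state as BP_Player enters or leaves.
; Entering turns on a vignette material on the player camera, flags both linked prone actors as InsideConduit and opens their Cube1 collision.
; Leaving zeroes the vignette, calls CrawlingSystem, re-blocks both cubes and sets walk speed and camera yaw limits.
; Both responses require a PostProcessVolume in the level.
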(event OnComponentEndOverlap(Box)
  (params (OverlappedComponent :type Primitive%20Component%20Object%20Reference) (OtherActor :type Actor%20Object%20Reference) (OtherComp :type Primitive%20Component%20Object%20Reference) (OtherBodyIndex :type Integer))
  (bind _returnvalue (Game|GetPlayerCameraManager 0))
  (bind _ref_prone (Variables|Default|GetRef_Prone))
  (bind _cube1 (Variables|/Game/Blueprints/BP_Object/BP_Prone.BP_Prone_C|GetCube1 _ref_prone))
  (bind _asbp_player (Utilities|Casting|CastToBP_Player OtherActor))
  (bind _returnvalue_2 (Rendering|Material|CreateDynamicMaterialInstance "/Game/Jules/Material_Jules/PP_Vignette_Inst.PP_Vignette_Inst" "None" "None" :!class /Script/Engine.KismetMaterialLibrary))
  (Variables|/Game/Blueprints/BP_Player.BP_Player_C|SetPostPocessDamageDynamicMaterial _asbp_player _returnvalue_2)
  (bind _returnvalue_3 (Actor|GetActorOfClass "/Script/Engine.PostProcessVolume"))
  (Utilities|IsValid _returnvalue_3
    (:Is%20Valid
      (Utilities|Array|SetArrayElem (Utilities|Struct|BreakWeightedBlendables (Utilities|Struct|BreakPostProcessSettings (Variables|/Script/Engine.CameraComponent|GetPostProcessSettings (Variables|/Game/Blueprints/BP_Player.BP_Player_C|GetCamera _asbp_player)))) 6 (Utilities|Array|Get(acopy) (Utilities|Array|MakeArray (Utilities|Struct|MakeWeightedBlendable 0.0 (Variables|/Game/Blueprints/BP_Player.BP_Player_C|GetPostPocessDamageDynamicMaterial _asbp_player)))))
      (Default|CrawlingSystem _asbp_player)
      (Variables|/Game/Blueprints/BP_Object/BP_Prone.BP_Prone_C|SetInsideConduit (Variables|Default|GetRef_Prone) false)
      (Variables|/Game/Blueprints/BP_Object/BP_Prone.BP_Prone_C|SetInsideConduit (Variables|Default|GetRef_Prone2) false)
      (Collision|SetCollisionResponsetoChannel _cube1 "ECC_Pawn" "ECR_Block")
      (Collision|SetCollisionResponsetoChannel _cube1 "ECC_Visibility" "ECR_Block")
      ;[0.5819 1 0.5801] Increase Speed
      (Variables|/Script/Engine.CharacterMovementComponent|SetMaxWalkSpeed (Variables|/Script/Engine.Character|GetCharacterMovement _asbp_player) 225.0)
      ;[0.6927 0.2915 0.5435] Normal View
      (Variables|/Script/Engine.PlayerCameraManager|SetViewYawMin _returnvalue -179.0)
      (Variables|/Script/Engine.PlayerCameraManager|SetViewYawMax _returnvalue 179.0))))

(event OnComponentBeginOverlap(Box)
  (params (OverlappedComponent :type Primitive%20Component%20Object%20Reference) (OtherActor :type Actor%20Object%20Reference) (OtherComp :type Primitive%20Component%20Object%20Reference) (OtherBodyIndex :type Integer) (bFromSweep :type Boolean) (SweepResult :type Hit%20Result%20Structure%20%28by%20ref%29))
  (bind _ref_prone (Variables|Default|GetRef_Prone))
  (bind _cube1 (Variables|/Game/Blueprints/BP_Object/BP_Prone.BP_Prone_C|GetCube1 _ref_prone))
  (bind _asbp_player (Utilities|Casting|CastToBP_Player OtherActor))
  (bind _returnvalue (Rendering|Material|CreateDynamicMaterialInstance "/Game/Jules/Material_Jules/PP_Vignette_Inst.PP_Vignette_Inst" "None" "None" :!class /Script/Engine.KismetMaterialLibrary))
  (Variables|/Game/Blueprints/BP_Player.BP_Player_C|SetPostPocessDamageDynamicMaterial _asbp_player _returnvalue)
  (bind _returnvalue_2 (Actor|GetActorOfClass "/Script/Engine.PostProcessVolume"))
  (Utilities|IsValid _returnvalue_2
    (:Is%20Valid
      (Utilities|Array|SetArrayElem (Utilities|Struct|BreakWeightedBlendables (Utilities|Struct|BreakPostProcessSettings (Variables|/Script/Engine.CameraComponent|GetPostProcessSettings (Variables|/Game/Blueprints/BP_Player.BP_Player_C|GetCamera _asbp_player)))) 6 (Utilities|Array|Get(acopy) (Utilities|Array|MakeArray (Utilities|Struct|MakeWeightedBlendable 1.0 (Variables|/Game/Blueprints/BP_Player.BP_Player_C|GetPostPocessDamageDynamicMaterial _asbp_player)))))
      (Variables|/Game/Blueprints/BP_Object/BP_Prone.BP_Prone_C|SetInsideConduit _ref_prone true)
      (Variables|/Game/Blueprints/BP_Object/BP_Prone.BP_Prone_C|SetInsideConduit (Variables|Default|GetRef_Prone2) true)
      (Collision|SetCollisionResponsetoChannel _cube1 "ECC_Pawn" "ECR_Overlap")
      (Collision|SetCollisionResponsetoChannel _cube1 "ECC_Visibility" "ECR_Ignore"))))

(event EventTick
  (params (DeltaSeconds :type Float%20%28single-precision%29)))

(fn ConstructionScript)