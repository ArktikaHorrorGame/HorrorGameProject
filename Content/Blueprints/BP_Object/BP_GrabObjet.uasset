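; Grabbable physics object that makes impact noise and manages its collision with the player.
; Player hits set the character's physics interaction from CanBePush.
; Other hits, throttled by timers that also mute the first impact, play a sound and report a noise event when any signed velocity axis exceeds a threshold.
; For light objects, a box overlap ignores Pawn collision while grabbed and restores blocking on exit.
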(event OnComponentBeginOverlap(Box)
  (params (OverlappedComponent :type Primitive%20Component%20Object%20Reference) (OtherActor :type Actor%20Object%20Reference) (OtherComp :type Primitive%20Component%20Object%20Reference) (OtherBodyIndex :type Integer) (bFromSweep :type Boolean) (SweepResult :type Hit%20Result%20Structure%20%28by%20ref%29))
  ;[0.1979 0.06391 0.07982] Disable Collision when object is touching the player
  (Utilities|Casting|CastToBP_Player OtherActor)
  (switch Utilities|FlowControl|Switch|SwitchonE_ObjectType (Variables|Default|GetObject_Type)
    (:NewEnumerator1
      (if (Variables|Default|GetGrabbed?)
        (Development|PrintString "Object touch player WHILE grabbing it")
        (Collision|SetCollisionResponsetoChannel (Variables|Debug|GetStaticMeshComponent) "ECC_Pawn" "ECR_Ignore")))))

(event OnComponentEndOverlap(Box)
  (params (OverlappedComponent :type Primitive%20Component%20Object%20Reference) (OtherActor :type Actor%20Object%20Reference) (OtherComp :type Primitive%20Component%20Object%20Reference) (OtherBodyIndex :type Integer))
  (bind _staticmeshcomponent (Variables|Debug|GetStaticMeshComponent))
  ;[0.1979 0.06391 0.07982] Disable Collision when object is touching the player
  (Utilities|Casting|CastToBP_Player OtherActor)
  (switch Utilities|FlowControl|Switch|SwitchonE_ObjectType (Variables|Default|GetObject_Type)
    (:NewEnumerator1
      (if (Variables|Default|GetGrabbed?)
        (Development|PrintString "Object leave player WHILE grabbing  it")
        (Collision|SetCollisionResponsetoChannel _staticmeshcomponent "ECC_Pawn" "ECR_Block")
        (else
          (Development|PrintString "Object leave player WITHOUT grabbing it ")
          (Collision|SetCollisionResponsetoChannel _staticmeshcomponent "ECC_Pawn" "ECR_Block"))))))

(event OnComponentHit(StaticMeshComponent)
  (params (HitComponent :type Primitive%20Component%20Object%20Reference) (OtherActor :type Actor%20Object%20Reference) (OtherComp :type Primitive%20Component%20Object%20Reference) (NormalImpulse :type Vector :default "0, 0, 0") (Hit :type Hit%20Result%20Structure%20%28by%20ref%29))
  (bind _staticmeshcomponent (Variables|Debug|GetStaticMeshComponent))
  (bind _returnvalue (Transformation|GetWorldLocation _staticmeshcomponent))
  (bind _asbp_player (Utilities|Casting|CastToBP_Player OtherActor)
    (:then
      (Variables|/Script/Engine.CharacterMovementComponent|SetbEnablePhysicsInteraction (Variables|/Script/Engine.Character|GetCharacterMovement _asbp_player) (Variables|Default|GetCanBePush?)))
    (:CastFailed
      (if (Variables|Default|GetFirstSound?)
        (Variables|Default|SetFirstSound? false)
        (Utilities|Time|SetTimerbyEvent (delegate Custom|MakeSound) 1.0)
        (Variables|Default|SetDoSound? false)
        (elif (Variables|Default|GetDoSound?)
          (Utilities|Time|SetTimerbyEvent (delegate Custom|MakeSound) 0.2)
          (Variables|Default|SetDoSound? false)
          (bind _outhit (Collision|SphereTraceByChannel _returnvalue _returnvalue 3e+01 "TraceTypeQuery1" true 0 "ForDuration"))
          (bind _returnvalue_2 (Physics|GetPhysicsLinearVelocity (Variables|Debug|GetStaticMeshComponent) "None"))
          (if (Math|Boolean|ORBoolean (> (.x _returnvalue_2) 65.0) (> (.y _returnvalue_2) 65.0) (> (.z _returnvalue_2) 65.0))
            (Audio|SpawnSoundatLocation (Variables|Default|GetSound) (.location _outhit) "0, 0, 0" 1.0 1.0 0.0 0 0)
            (Class|AISenseHearing|ReportNoiseEvent (.location _outhit) 1.0 self 3e+03 (Utilities|Name|EnumtoName (Variables|Default|GetSound_Type)))))))))

(event Custom|MakeSound
  (Variables|Default|SetDoSound? true))

(event EventGrabed
  (params (GrabPoint_Location :type Scene%20Component%20Object%20Reference) (Cam%20/Camera%20Arm :type Spring%20Arm%20Component%20Object%20Reference) (BP_Player_Ref :type BP%20Player%20Object%20Reference))
  (Variables|Default|SetGrabbed? true))

(event EventReleased
  (Variables|Default|SetGrabbed? false))

(fn ConstructionScript)