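; BP_Cube is a grabbable metal cube that makes sounds and reports AI-audible noise attributed to the player.
; The first grab plays a metal sound with a short-range noise event; that DoOnce is never reset, and release does nothing.
; Mesh hits play a second sound with a much longer-range noise event, throttled by a DoOnce that resets after a brief delay.
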(event OnComponentHit(StaticMeshComponent1)
  (params (HitComponent :type Primitive%20Component%20Object%20Reference) (OtherActor :type Actor%20Object%20Reference) (OtherComp :type Primitive%20Component%20Object%20Reference) (NormalImpulse :type Vector :default "0, 0, 0") (Hit :type Hit%20Result%20Structure%20%28by%20ref%29))
  (bind _staticmeshcomponent1 (Variables|Default|GetStaticMeshComponent1))
  (bind _returnvalue (Transformation|GetWorldLocation _staticmeshcomponent1))
  (Utilities|FlowControl|DoOnce false :!label _label
    (:Completed
      (Audio|PlaySoundatLocation "/Game/Blueprints/Audio/Footsteps/Metal_02.Metal_02" _returnvalue "0, 0, 0" 1.0 1.0 0.0 0 0 0 0)
      (Class|AISenseHearing|ReportNoiseEvent _returnvalue 1.0 (Game|GetPlayerCharacter 0) 1e+04 "None")
      (Utilities|FlowControl|Delay 0.5)
      (goto _label Reset))))

(event EventReleased)

(event EventGrabed
  (bind _returnvalue (Transformation|GetActorLocation))
  (Utilities|FlowControl|DoOnce false
    (:Completed
      (Audio|PlaySoundatLocation "/Game/Blueprints/Audio/Footsteps/Metal_01.Metal_01" _returnvalue "0, 0, 0" 1.0 1.0 0.0 0 0 0 0)
      (Class|AISenseHearing|ReportNoiseEvent _returnvalue 1.0 (Game|GetPlayerCharacter 0) 1e+02 "None"))))

(fn ConstructionScript)