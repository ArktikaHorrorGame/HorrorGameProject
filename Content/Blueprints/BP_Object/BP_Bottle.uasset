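; BP_Bottle is a breakable bottle actor that shatters when it hits something at high speed.
; A Box component hit passes through a DoOnce, then compares the actor's velocity magnitude to a speed threshold.
; Above it, the bottle destroys itself and spawns ShatterBottle at its location and rotation.
; The DoOnce resets only on that shatter branch, so a slower first hit blocks later hit checks.
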(event OnComponentHit(Box)
  (params (HitComponent :type Primitive%20Component%20Object%20Reference) (OtherActor :type Actor%20Object%20Reference) (OtherComp :type Primitive%20Component%20Object%20Reference) (NormalImpulse :type Vector :default "0, 0, 0") (Hit :type Hit%20Result%20Structure%20%28by%20ref%29))
  (Utilities|FlowControl|DoOnce false :!label _label
    (:Completed
      (if (>= (Math|Vector|VectorLength (Transformation|GetVelocity)) 6.5e+02)
        (Actor|DestroyActor)
        (Game|SpawnActorfromClass "/Game/FirstPerson/AllMeca/Chaos/ShatterBottle.ShatterBottle_C" (Math|Transform|MakeTransform (Transformation|GetActorLocation) (Transformation|GetActorRotation) "1.000000,1.000000,1.000000") "Undefined" "MultiplyWithRoot" 0 0)
        (goto _label Reset)))))

(event Collision|EventActorBeginOverlap
  (params (OtherActor :type Actor%20Object%20Reference)))

(event Game|Damage|EventAnyDamage
  (params (Damage :type Float%20%28single-precision%29) (DamageType :type Damage%20Type%20Object%20Reference) (InstigatedBy :type Controller%20Object%20Reference) (DamageCauser :type Actor%20Object%20Reference)))

(event EventTick
  (params (DeltaSeconds :type Float%20%28single-precision%29)))

(fn ConstructionScript
  (|CallParentFunction))