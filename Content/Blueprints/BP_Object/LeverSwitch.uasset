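; LeverSwitch is a physics-driven two-position lever that switches a linked object on or off.
; Its lever check, run from Tick, reads the handle's roll relative to the actor.
; That roll picks the physics constraint's angular target on either side of center, so the lever settles into one of two positions.
; The same threshold sends activate or deactivate messages to a valid LinkedObject on every check, not only on changes.
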(event Custom|Lever_Check
  (bind _returnvalue (Transformation|GetActorTransform))
  (bind _handle (Variables|Default|GetHandle))
  (bind _linkedobject (Variables|Default|GetLinkedObject))
  (bind _returnvalue_2 (Transformation|GetWorldRotation _handle))
  (bind _returnvalue_3 (Math|Transform|InverseTransformRotation _returnvalue _returnvalue_2))
  (bind _roll (Math|Rotator|BreakRotator _returnvalue_3))
  (bind _returnvalue_4 (< _roll 2e+01))
  (Class|PhysicsConstraintComponent|SetAngularOrientationTarget (Variables|Default|GetPhysicsConstraint) (Math|Rotator|MakeRotator (Math|Float|SelectFloat -45.0 45.0 _returnvalue_4) 0.0 0.0))
  (Variables|Default|GetLinkedObject
    (:then
      (if _returnvalue_4
        (Class|BPIObjectActivate|ObjectActivate(Message) _linkedobject)
        (else
          (Class|BPIObjectActivate|ObjectDesactivate(Message) _linkedobject))))
    (:else)))

(event EventTick
  (params (DeltaSeconds :type Float%20%28single-precision%29))
  (CallFunction|LeverCheck))

(fn ConstructionScript)