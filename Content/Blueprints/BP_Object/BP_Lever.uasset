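; BP_Lever is a physics-hinged lever that switches a linked object on or off.
; Every tick it runs a lever check that reads the sign of the main mesh's world roll.
; The hinge constraint's angular target follows that sign, pulling the lever toward one of two opposite angles for bistable snapping.
; The linked object receives an activate or deactivate message on each check, not only on state changes.
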(event Custom|Lever_Check
  (bind _linkedobject (Variables|Default|GetLinkedObject))
  (bind _mainmesh (Variables|Default|GetMainMesh))
  (bind _returnvalue (Transformation|GetWorldRotation _mainmesh))
  (bind _roll (Math|Rotator|BreakRotator _returnvalue))
  (bind _returnvalue_2 (< _roll 0.0))
  (Class|PhysicsConstraintComponent|SetAngularOrientationTarget (Variables|Default|GetHinges) (Math|Rotator|MakeRotator (Math|Float|SelectFloat -45.0 45.0 _returnvalue_2) 0.0 0.0))
  (if _returnvalue_2
    (Class|BPILeverActivate|LeverActivate(Message) _linkedobject)
    (else
      (Class|BPILeverActivate|LeverDesactivate(Message) _linkedobject))))

(event EventBeginPlay
  (|CallParentFunction) ; This node is disabled and will not be called.\nDrag off pins to build functionality.
)

(event Collision|EventActorBeginOverlap
  (params (OtherActor :type Actor%20Object%20Reference)))

(event EventTick
  (params (DeltaSeconds :type Float%20%28single-precision%29))
  (CallFunction|LeverCheck)
  (|CallParentFunction DeltaSeconds))

(fn ConstructionScript
  (|CallParentFunction))