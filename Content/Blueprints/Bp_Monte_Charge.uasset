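; Freight elevator (monte-charge) that the player operates through an Interaction event, usable only when the FusibleBon fuse flag is true.
; Each interaction locks player movement and alternates through a FlipFlop between playing and reversing a timeline.
; The timeline lerps the platform mesh between the BMonteCharge and HMonteCharge locations, with play rate derived from TDeplacement, and restores player movement on finish.
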(event Custom|Elevate_elavator
  (bind _elevator (Timeline|Timeline Play)
    (:Update
      (Transformation|SetWorldLocation (Variables|Default|GetStaticMeshComponent1) (Math|Vector|Lerp(Vector) (Transformation|GetWorldLocation (Variables|Default|GetB_Monte_Charge)) (Transformation|GetWorldLocation (Variables|Default|GetH_Monte_Charge)) _elevator) false false))
    (:Finished
      (Variables|/Game/Blueprints/BP_Player.BP_Player_C|SetCan_Move? (.AsBP%20Player (Utilities|Casting|CastToBP_Player (Game|GetPlayerCharacter 0))) true))))

(event Custom|Reverse_elevator
  (Audio|Components|Audio|Stop (Variables|Default|GetTimeline))
  (bind _elevator (Timeline|Timeline Reverse)
    (:Update
      (Transformation|SetWorldLocation (Variables|Default|GetStaticMeshComponent1) (Math|Vector|Lerp(Vector) (Transformation|GetWorldLocation (Variables|Default|GetB_Monte_Charge)) (Transformation|GetWorldLocation (Variables|Default|GetH_Monte_Charge)) _elevator) false false))
    (:Finished
      (Variables|/Game/Blueprints/BP_Player.BP_Player_C|SetCan_Move? (.AsBP%20Player (Utilities|Casting|CastToBP_Player (Game|GetPlayerCharacter 0))) true))))

(event EventBeginPlay
  (Components|Timeline|SetPlayRate (Variables|Default|GetTimeline) (/ 1.0 (Variables|Default|GetT_Deplacement))))

(event EventInteraction
  (if (Variables|Default|GetFusible_Bon?)
    (Variables|/Game/Blueprints/BP_Player.BP_Player_C|SetCan_Move? (.AsBP%20Player (Utilities|Casting|CastToBP_Player (Game|GetPlayerCharacter 0))) false)
    (Utilities|FlowControl|FlipFlop
      (:A
        (CallFunction|ElevateElavator))
      (:B
        (CallFunction|ReverseElevator)))))

(fn ConstructionScript)