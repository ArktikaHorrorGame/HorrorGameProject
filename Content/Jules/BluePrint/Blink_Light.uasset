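; Blink_Light is an actor whose point light flickers irregularly.
; Tick runs a random Delay of up to one second, then toggles the light's visibility.
; BeginPlay starts a looping Blackout timer, but that event and LigthOn are empty.
; Disconnected nodes hold unfinished blackout logic that would cut the light's intensity and schedule its restoration.
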(event Custom|Blackout)

(event Custom|LigthOn)

(event EventBeginPlay
  (Utilities|Time|SetTimerbyFunctionName 0 "Blackout " 3e+01 true))

(event Collision|EventActorBeginOverlap
  (params (OtherActor :type Actor%20Object%20Reference)))

(event EventTick
  (params (DeltaSeconds :type Float%20%28single-precision%29))
  (Utilities|FlowControl|Delay (Math|Random|RandomFloatinRange 0.1 1.0))
  (Rendering|ToggleVisibility (Variables|Default|GetPointLight) false))

(fn ConstructionScript)