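; BP_FlashBang applies and clears a flashbang screen effect through post-process settings on the BP_Player camera.
; FlashBang sets the flashbang material's blend weight to full and spikes an intensity setting, while DeleteFlash reverses both.
; WhiteFlash only spikes the intensity.
; FlashBangEffect only sets the material, if a PostProcessVolume exists, and prints debug text, but never edits that volume.
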(event Custom|WhiteFlash
  (bind _returnvalue (Game|GetPlayerCharacter 0))
  (bind _asbp_player (Utilities|Casting|CastToBP_Player _returnvalue))
  (bind _camera (Variables|/Game/Blueprints/BP_Player.BP_Player_C|GetCamera _asbp_player))
  (bind _structout (Utilities|Struct|SetmembersinPostProcessSettings (Variables|/Script/Engine.CameraComponent|GetPostProcessSettings _camera) 250.675))
  (Variables|/Script/Engine.CameraComponent|SetPostProcessSettings _camera _structout))

(event Custom|FlashBang%20Effect
  (bind _returnvalue (Actor|GetActorOfClass "/Script/Engine.PostProcessVolume"))
  (Utilities|IsValid _returnvalue
    (:Is%20Valid
      (Utilities|Array|SetArrayElem (Utilities|Struct|BreakWeightedBlendables (Utilities|Struct|BreakPostProcessSettings (Variables|/Script/Engine.CameraComponent|GetPostProcessSettings (Variables|/Game/Blueprints/BP_Player.BP_Player_C|GetCamera (.AsBP%20Player (Utilities|Casting|CastToBP_Player (Game|GetPlayerCharacter 0))))))) 0 (Utilities|Array|Get(acopy) (Utilities|Array|MakeArray (Utilities|Struct|MakeWeightedBlendable 1.0 "/Game/Jules/PostProcessMAterial/M_PostProcess_FlashBang_Inst.M_PostProcess_FlashBang_Inst"))))
      (Development|PrintString "Hello"))))

(event Custom|FlashBang
  (bind _returnvalue (Game|GetPlayerCharacter 0))
  (bind _asbp_player (Utilities|Casting|CastToBP_Player _returnvalue))
  (bind _camera (Variables|/Game/Blueprints/BP_Player.BP_Player_C|GetCamera _asbp_player))
  (Utilities|Array|SetArrayElem (Utilities|Struct|BreakWeightedBlendables (Utilities|Struct|BreakPostProcessSettings (Variables|/Script/Engine.CameraComponent|GetPostProcessSettings _camera))) 0 (Utilities|Array|Get(acopy) (Utilities|Array|MakeArray (Utilities|Struct|MakeWeightedBlendable 1.0 "/Game/Jules/PostProcessMAterial/M_PostProcess_FlashBang_Inst.M_PostProcess_FlashBang_Inst"))))
  (bind _structout (Utilities|Struct|SetmembersinPostProcessSettings (Variables|/Script/Engine.CameraComponent|GetPostProcessSettings _camera) 250.675))
  (Variables|/Script/Engine.CameraComponent|SetPostProcessSettings _camera _structout))

(event Custom|DeleteFlash
  (bind _returnvalue (Game|GetPlayerCharacter 0))
  (bind _asbp_player (Utilities|Casting|CastToBP_Player _returnvalue))
  (bind _camera (Variables|/Game/Blueprints/BP_Player.BP_Player_C|GetCamera _asbp_player))
  (Utilities|Array|SetArrayElem (Utilities|Struct|BreakWeightedBlendables (Utilities|Struct|BreakPostProcessSettings (Variables|/Script/Engine.CameraComponent|GetPostProcessSettings _camera))) 0 (Utilities|Array|Get(acopy) (Utilities|Array|MakeArray (Utilities|Struct|MakeWeightedBlendable 0.0 "/Game/Jules/PostProcessMAterial/M_PostProcess_FlashBang_Inst.M_PostProcess_FlashBang_Inst"))))
  (bind _structout (Utilities|Struct|SetmembersinPostProcessSettings (Variables|/Script/Engine.CameraComponent|GetPostProcessSettings _camera) 0.675))
  (Variables|/Script/Engine.CameraComponent|SetPostProcessSettings _camera _structout))

(event EventBeginPlay)

(event Collision|EventActorBeginOverlap
  (params (OtherActor :type Actor%20Object%20Reference)))

(event EventTick
  (params (DeltaSeconds :type Float%20%28single-precision%29)))

(fn ConstructionScript)