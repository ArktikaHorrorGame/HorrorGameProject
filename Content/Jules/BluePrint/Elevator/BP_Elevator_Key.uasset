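; BP_Elevator_Key is a key receptacle that registers two specific keys with an elevator.
; When a BP_Valve_Key overlaps its Box, it compares that actor against its Key1 and Key2 references.
; A match sets the corresponding flag on the Elevator, calls Release on the player, destroys the key and reveals the matching hidden fuse component.
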(event OnComponentBeginOverlap(Box)
  (params (OverlappedComponent :type Primitive%20Component%20Object%20Reference) (OtherActor :type Actor%20Object%20Reference) (OtherComp :type Primitive%20Component%20Object%20Reference) (OtherBodyIndex :type Integer) (bFromSweep :type Boolean) (SweepResult :type Hit%20Result%20Structure%20%28by%20ref%29))
  (bind _returnvalue (Game|GetPlayerCharacter 0))
  (bind _elevator (Variables|Default|GetElevator))
  (bind _asbp_valve_key (Utilities|Casting|CastToBP_Valve_Key OtherActor))
  (Variables|Default|SetAs%20BP%20Valve%20Key _asbp_valve_key)
  (if (== (Variables|Default|GetAs%20BP%20Valve%20Key) (Variables|Default|GetKey_1))
    (Variables|/Game/Jules/BluePrint/Elevator/BP_Elevator.BP_Elevator_C|SetKey1 _elevator true)
    (bind _asbp_player (Utilities|Casting|CastToBP_Player _returnvalue))
    (Default|Release _asbp_player)
    (Actor|DestroyActor (Variables|Default|GetKey_1))
    (Development|SetHiddeninGame (Variables|Default|Getfusibl) false false)
    (elif (== (Variables|Default|GetAs%20BP%20Valve%20Key) (Variables|Default|GetKey2))
      (Variables|/Game/Jules/BluePrint/Elevator/BP_Elevator.BP_Elevator_C|SetKey2 _elevator true)
      (bind _asbp_player_2 (Utilities|Casting|CastToBP_Player _returnvalue))
      (Default|Release _asbp_player_2)
      (Actor|DestroyActor (Variables|Default|GetKey2))
      (Development|SetHiddeninGame (Variables|Default|Getfusibl1) false false))))

(fn ConstructionScript)