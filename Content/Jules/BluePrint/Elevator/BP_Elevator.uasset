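; BP_Elevator is an elevator that rides only for a player holding both keys, otherwise printing a hint naming the missing key.
; Entering the Box trigger checks HasKey1 and then HasKey2 on BP_Player before playing the Elevator timeline, which drives the Cube's relative location.
; Leaving the box reverses the timeline, returning the platform along its path without checking keys.
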(event OnComponentBeginOverlap(Box)
  (params (OverlappedComponent :type Primitive%20Component%20Object%20Reference) (OtherActor :type Actor%20Object%20Reference) (OtherComp :type Primitive%20Component%20Object%20Reference) (OtherBodyIndex :type Integer) (bFromSweep :type Boolean) (SweepResult :type Hit%20Result%20Structure%20%28by%20ref%29))
  (bind _asbp_player (Utilities|Casting|CastToBP_Player OtherActor))
  (if (Variables|/Game/Blueprints/BP_Player.BP_Player_C|GetHasKey%201 _asbp_player)
    (if (Variables|/Game/Blueprints/BP_Player.BP_Player_C|GetHasKey%202 _asbp_player)
      (bind _elevator (Timeline|Elevator Play)
        (:Update
          (Transformation|SetRelativeLocation (Variables|Default|GetCube) _elevator false false)))
      (else
        (Development|PrintString "Search key 2 ! ")))
    (else
      (Development|PrintString "Search key 1 ! "))))

(event OnComponentEndOverlap(Box)
  (params (OverlappedComponent :type Primitive%20Component%20Object%20Reference) (OtherActor :type Actor%20Object%20Reference) (OtherComp :type Primitive%20Component%20Object%20Reference) (OtherBodyIndex :type Integer))
  (Utilities|Casting|CastToBP_Player OtherActor)
  (bind _elevator (Timeline|Elevator Reverse)
    (:Update
      (Transformation|SetRelativeLocation (Variables|Default|GetCube) _elevator false false))))

(fn ConstructionScript)