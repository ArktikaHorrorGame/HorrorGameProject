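; Toxic gas jet hazard that knocks the player back and can be blocked by heavy objects.
; Each tick, a line trace along the Niagara up vector detects what the jet hits.
; A player hit triggers a timer-reset DoOnce that launches them horizontally and flashes a damage post-process, later faded by a timeline.
; A BP_Objet_Lourd hit scales gas and distortion particle lifetime by hit distance, shortening the jet.
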(event Custom|Delete_Post_Pro
  (bind _newtrack_0 (Timeline|Timeline PlayFromStart)
    (:Update
      (Rendering|Material|SetScalarParameterValue (Variables|/Game/Blueprints/BP_Player.BP_Player_C|GetPostPocessDamageDynamicMaterial (stale Custom|Detect%20Object _asbp_player)) "Intensity" (Math|Float|Lerp 1.0 0.0 _newtrack_0) :!class /Script/Engine.MaterialInstanceDynamic))))

(event Custom|Detect%20Object
  (bind _niagara (Variables|Default|GetNiagara))
  (bind _returnvalue (Transformation|GetWorldLocation _niagara))
  (bind (_outhit _returnvalue_2) (Collision|LineTraceByChannel _returnvalue (+ _returnvalue (* (Math|Vector|GetUpVector _niagara) (Variables|Default|GetLT_Distance))) "TraceTypeQuery2" false 0 "Persistent" false))
  (if _returnvalue_2
    (Variables|Default|SetDistance (.Distance (Collision|BreakHitResult _outhit)))
    (bind _asbp_player (Utilities|Casting|CastToBP_Player (.HitActor (Collision|BreakHitResult _outhit)))
      (:then
        (Utilities|FlowControl|DoOnce false
          (:Completed
            (CallFunction|PushPlayer _asbp_player (.Location (Collision|BreakHitResult _outhit)))
            (Utilities|Time|SetTimerbyEvent (delegate Custom|Delete_Post_Pro) 2.0)
            (Utilities|Time|SetTimerbyEvent (delegate Custom|Reset%20Push) 0.5))))
      (:CastFailed
        (Utilities|Casting|CastToBP_Objet_Lourd (.HitActor (Collision|BreakHitResult _outhit)))
        (CallFunction|CalculNewLifeTime)
        (Effects|Components|ParticleSystem|SetFloatParameter (Variables|Default|GetNiagara) "LifeTime" (Variables|Default|GetNew_LifeTime))
        (Effects|Components|ParticleSystem|SetFloatParameter (Variables|Default|GetDistortion) "LifeTime" (Variables|Default|GetNew_LifeTime))))))

(event Custom|Reset%20Push
  (Utilities|FlowControl|DoOnce false) ; enters at Reset
)

(event EventTick
  (params (DeltaSeconds :type Float%20%28single-precision%29))
  (CallFunction|DetectObject))

(fn ConstructionScript)

(fn CalculNewLifeTime
  (Variables|Default|SetNew_LifeTime (/ (* (Variables|Default|GetMax_LifeTime) (Variables|Default|GetDistance)) (Variables|Default|GetLT_Distance))))

(fn PushPlayer
  (params (Player :type BP%20Player%20Object%20Reference) (NewParam :type Vector))
  (bind _returnvalue (Game|GetPlayerCharacter 0))
  (bind _launch_player (Variables|Default|GetLaunch_player))
  (bind _mesh (Variables|/Script/Engine.Character|GetMesh _returnvalue))
  (bind _returnvalue_2 (Transformation|GetWorldLocation _mesh))
  (bind _returnvalue_3 (Math|Rotator|FindLookatRotation NewParam _returnvalue_2))
  (bind _returnvalue_4 (Math|Vector|GetForwardVector _returnvalue_3))
  (bind _returnvalue_5 (* _returnvalue_4 _launch_player))
  (bind (_x _y) (Math|Vector|BreakVector _returnvalue_5))
  (Character|LaunchCharacter Player (Math|Vector|MakeVectorNetQuantize _x _y 0.0) true true)
  (Rendering|Material|SetScalarParameterValue (Variables|/Game/Blueprints/BP_Player.BP_Player_C|GetPostPocessDamageDynamicMaterial Player) "Intensity" 1.0 :!class /Script/Engine.MaterialInstanceDynamic))